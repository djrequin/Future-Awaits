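; Corrupted obstacle that stays closed until its linked flowers die, then can be destroyed by a shot.
; On BeginPlay it registers itself with each flower; Death events advance a counter, and the final one marks it weak and plays an opening montage.
; ShotEvent then spawns a dark-magic Niagara effect and destroys the actor.
; When it contains goals and the quest is active, both stages update the game mode's goal.
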(event Custom|Death
  (bind _as_bp_third_person_game_mode (Variables|Default|GetAs%20BP%20Third%20Person%20Game%20Mode))
  (Math|Integer|IncrementInt (Variables|Default|GetLine)
    (:%20%20
      (Utilities|IsValid _as_bp_third_person_game_mode
        (:Is%20Valid
          (if (Variables|Default|GetIs%20quest%20activated?)
            (Default|ChangeGoal _as_bp_third_person_game_mode (Utilities|Array|Get(acopy) (Variables|Goals|GetGoals) (- (Variables|Default|GetLine) 1)) "NewEnumerator0")))
        (:Is%20Not%20Valid
          _))
      (if (>= (Variables|Default|GetLine) (Utilities|Array|Length (Variables|Default|GetFlowers)))
        (Variables|Default|SetIs_Weak true)
        (Animation|Montage|PlayMontage (Variables|Default|GetSkeletalMesh) "/Game/Prototypage/Corrupted_flowers/Anims/Big_Flower/NewFolder/Opening_Montage.Opening_Montage"
          (:OnCompleted
            (Development|PrintString "opened")))))))

(event EventBeginPlay
  (for _array_element (Variables|Default|GetFlowers)
    (Variables|/Game/Prototypage/Corrupted_flowers/BP_Corrupted_Flower.BP_Corrupted_Flower_C|SetObstacle _array_element self)
    (if (Variables|Goals|GetContains_goals%20?)
      (bind _asbp_third_person_game_mode (Utilities|Casting|CastToBP_ThirdPersonGameMode (Game|GetGameMode)))
      (Variables|Default|SetAs%20BP%20Third%20Person%20Game%20Mode _asbp_third_person_game_mode))))

(event Collision|EventActorBeginOverlap
  (params (OtherActor :type Actor%20Object%20Reference)))

(event EventTick
  (params (DeltaSeconds :type Float%20%28single-precision%29)))

(event EventShotEvent
  (params (Impact_Location :type Vector :default "0, 0, 0"))
  (bind _returnvalue (Transformation|GetActorLocation))
  (bind _as_bp_third_person_game_mode (Variables|Default|GetAs%20BP%20Third%20Person%20Game%20Mode))
  (if (Variables|Default|GetIs_Weak)
    (Niagara|SpawnSystematLocation "/Game/BlinkAndDashVFX/VFX_Niagara/NS_Blink_DarkMagic.NS_Blink_DarkMagic" (Math|Vector|MakeVector (.x _returnvalue) (.y _returnvalue) (+ (.z _returnvalue) 3.5e+02)) "0, 0, 0" (Math|Conversions|ToVector(Float) (Variables|Default|GetNewVar)))
    (Actor|DestroyActor)
    (Utilities|IsValid _as_bp_third_person_game_mode
      (:Is%20Valid
        (if (Variables|Default|GetIs%20quest%20activated?)
          (Default|ChangeGoal _as_bp_third_person_game_mode (Utilities|Array|Get(acopy) (Variables|Goals|GetGoals) (Variables|Default|GetLine)) "NewEnumerator1")
          (Utilities|IsValid (Variables|Default|GetQuest_Starting_Point)))))))

(fn ConstructionScript)