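; BP_Corrupted_Flower is a shootable corrupted flower that clears a linked obstacle when destroyed.
; Its ShotEvent runs once, playing a 2D break sound, calling Death on the referenced Obstacle and destroying every valid actor in its Trace array.
; The flower then destroys itself and spawns a dark-magic Niagara effect at its location.
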(event EventBeginPlay)

(event Collision|EventActorBeginOverlap
  (params (OtherActor :type Actor%20Object%20Reference)))

(event EventTick
  (params (DeltaSeconds :type Float%20%28single-precision%29)))

(event EventShotEvent
  (Utilities|FlowControl|DoOnce false
    (:Completed
      (Audio|SpawnSound2D "/Game/Sounds/Corrupted_flowers/BREAK_FLOWER.BREAK_FLOWER" 1.0 1.0 0.0 0)
      (Default|Death (Variables|Default|GetObstacle))
      (for _array_element (Variables|Default|GetTrace)
        (Utilities|IsValid _array_element
          (:Is%20Valid
            (Actor|DestroyActor _array_element))))
      (Actor|DestroyActor)
      (Niagara|SpawnSystematLocation "/Game/BlinkAndDashVFX/VFX_Niagara/NS_Blink_DarkMagic.NS_Blink_DarkMagic" (Transformation|GetActorLocation)))))

(fn ConstructionScript)