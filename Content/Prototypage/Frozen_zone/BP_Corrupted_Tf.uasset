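; BP_Corrupted_Tf is a corrupted Time Fragment pickup that must be cleared of enemies before collection.
; The first interaction applies the locked material and spawns patrolling BP_Shadows at cached marker-sphere locations, linking each back to the fragment.
; When the kill count matches the Manager's enemy number, All_Ennemies_Dead? unlocks it and swaps the material.
; A later interaction increments the player's corrupted fragment count, destroys the actor and has the Manager verify fragments.
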(event Custom|Get_Locations
  (Utilities|FlowControl|Sequence
    (:then_0
      (Utilities|Array|Add (Variables|Default|GetSpheres_Locations) (Transformation|GetWorldLocation (Variables|Default|GetSphere1))))
    (:then_1
      (Utilities|Array|Add (Variables|Default|GetSpheres_Locations) (Transformation|GetWorldLocation (Variables|Default|GetSphere2))))
    (:then_2
      (Utilities|Array|Add (Variables|Default|GetSpheres_Locations) (Transformation|GetWorldLocation (Variables|Default|GetSphere3))))
    (:then_3
      (Utilities|Array|Add (Variables|Default|GetSpheres_Locations) (Transformation|GetWorldLocation (Variables|Default|GetSphere4))))))

(event Custom|All_Ennemies_Dead?
  (if (== (Variables|Default|GetEnnemies_Killed) (Variables|/Game/Prototypage/Frozen_zone/BP_Frozen_Zone_Manager.BP_Frozen_Zone_Manager_C|GetEnnemies_Number (Variables|Default|GetManager)))
    (Variables|Default|SetFirst_Time? false)
    (Rendering|Material|SetMaterial (Variables|Default|GetSphere) 0 "/Game/Prototypage/Materials/M_Corrupted_TimeFragmentsMaterial.M_Corrupted_TimeFragmentsMaterial")))

(event Custom|Bring
  (bind _asbp_third_person_character (Utilities|Casting|CastToBP_ThirdPersonCharacter (Game|GetPlayerCharacter 0)))
  (Variables|Default|SetAs%20BP%20Third%20Person%20Character _asbp_third_person_character)
  (Utilities|FlowControl|DoOnce false
    (:Completed
      (bind _result (Math|Integer|IncrementInt (Variables|/Game/ThirdPerson/Blueprints/BP_ThirdPersonCharacter.BP_ThirdPersonCharacter_C|GetCorrupted_TF _asbp_third_person_character))
        (:%20%20
          (Variables|/Game/ThirdPerson/Blueprints/BP_ThirdPersonCharacter.BP_ThirdPersonCharacter_C|SetCorrupted_TF _asbp_third_person_character _result)
          (Actor|DestroyActor))))))

(event EventBeginPlay
  (|CallParentFunction)
  (CallFunction|GetLocations))

(event EventTick
  (params (DeltaSeconds :type Float%20%28single-precision%29))
  (|CallParentFunction DeltaSeconds) ; This node is disabled and will not be called.\nDrag off pins to build functionality.
)

(event EventInteraction
  (if (Variables|Default|GetFirst_Time?)
    (if (Variables|Default|GetCantSpam)
      (Variables|Default|SetCantSpam false)
      (Rendering|Material|SetMaterial (Variables|Default|GetSphere) 0 "/Game/Prototypage/Materials/M_Corrupted_LockedTimeFragmentsMaterial.M_Corrupted_LockedTimeFragmentsMaterial")
      (for _index (range 0 (Variables|Default|GetNumber%20of%20ennemies%20to%20spawn))
        (bind _returnvalue (Game|SpawnActorfromClass "/Game/Prototypage/Fight/BP_Shadows.BP_Shadows_C" (Math|Transform|MakeTransform (Utilities|Array|Get(acopy) (Variables|Default|GetSpheres_Locations) (Variables|Default|GetLength)) "0, 0, 0" "1.000000,1.000000,1.000000") "Undefined" "MultiplyWithRoot" 0 0))
        (Utilities|Array|Add (Variables|Default|GetSpawned_Ennemies) _returnvalue)
        (Default|Patrol _returnvalue)
        (Utilities|IsValid (Utilities|Array|Get(acopy) (Variables|Default|GetSpawned_Ennemies) (Variables|Default|GetLength))
          (:Is%20Valid
            (Variables|/Game/Prototypage/Fight/BP_Ennemy_parent.BP_Ennemy_parent_C|SetCorrupted_TF? (Utilities|Array|Get(acopy) (Variables|Default|GetSpawned_Ennemies) (Variables|Default|GetLength)) true)
            (Variables|/Game/Prototypage/Fight/BP_Ennemy_parent.BP_Ennemy_parent_C|SetCorrupted_TF (Utilities|Array|Get(acopy) (Variables|Default|GetSpawned_Ennemies) (Variables|Default|GetLength)) self)
            (bind _result (Math|Integer|IncrementInt (Variables|Default|GetLength))
              (:%20%20
                (Variables|Default|SetLength _result)))))))
    (else
      (CallFunction|Bring)
      (Default|VerifyTF (Variables|Default|GetManager)))))

(fn ConstructionScript
  (|CallParentFunction))