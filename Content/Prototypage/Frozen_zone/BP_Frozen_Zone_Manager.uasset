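; Prototype frozen-zone manager that restarts its zone and rewards the player when corrupted objectives are cleared.
; After a delay at BeginPlay the sphere is rescaled; player overlap initializes the flagged objective type.
; Only corrupted time fragments get setup (manager reference, enemy count); the other two inits are empty.
; Verify events compare player counters to totals, then call RelancementDeLaZone and grant lucioles and time fragments through the HUD; Interaction restarts directly.
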(event OnComponentBeginOverlap(Sphere)
  (params (OverlappedComponent :type Primitive%20Component%20Object%20Reference) (OtherActor :type Actor%20Object%20Reference) (OtherComp :type Primitive%20Component%20Object%20Reference) (OtherBodyIndex :type Integer) (bFromSweep :type Boolean) (SweepResult :type Hit%20Result%20Structure%20%28by%20ref%29))
  ;[0 0 0] Changer réfs Player
  (Utilities|FlowControl|Sequence
    (:then_1
      (bind _asbp_third_person_character (Utilities|Casting|CastToBP_ThirdPersonCharacter OtherActor))
      (Variables|Default|SetAs%20BP%20Third%20Person%20Character _asbp_third_person_character)
      (CallFunction|Initialisation))))

(event Custom|Initialisation
  ;[0 0 0] Changer réfs Player
  (if (Variables|CorruptedTF|GetCorrupted_Time_Fragments)
    (CallFunction|1stInit)
    (elif (Variables|CorruptedFlowers|GetCorrupted_Flowers)
      (CallFunction|2ndInit)
      (elif (Variables|3rdOption|Get3rd_Option)
        (CallFunction|3rdInit)))))

(event Custom|3rd_Init
  ;[0 0 0] Changer réfs Player
)

(event Custom|1st_Init
  ;[0 0 0] Changer réfs Player
  ;;[1 0.1222 0] 2nd thing
  (for _array_element (Variables|CorruptedTF|GetCorrupted_TF)
    (Utilities|IsValid _array_element
      (:Is%20Valid
        (Variables|/Game/Prototypage/Frozen_zone/BP_Corrupted_Tf.BP_Corrupted_Tf_C|SetManager _array_element self)
        (Variables|/Game/Prototypage/Frozen_zone/BP_Corrupted_Tf.BP_Corrupted_Tf_C|SetNumber%20of%20ennemies%20to%20spawn _array_element (- (Variables|CorruptedTF|GetEnnemies_Number) 1))))))

(event Custom|Verify_TF
  ;[0 0 0] Changer réfs Player
  ;;[1 0.1222 0] 2nd thing
  (bind _asbp_third_person_character (Utilities|Casting|CastToBP_ThirdPersonCharacter (Game|GetPlayerCharacter 0)))
  (if (== (Variables|/Game/ThirdPerson/Blueprints/BP_ThirdPersonCharacter.BP_ThirdPersonCharacter_C|GetCorrupted_TF _asbp_third_person_character) (Utilities|Array|Length (Variables|CorruptedTF|GetCorrupted_TF)))
    (Default|RelancementDeLaZone (Variables|Default|GetManager))
    (CallFunction|Rewards)))

(event Custom|2nd_Init
  ;[0 0 0] Changer réfs Player
  ;;[0 1 0.1191] Flowers
)

(event Custom|rewards
  (bind _as_bp_third_person_character (Variables|Default|GetAs%20BP%20Third%20Person%20Character))
  (bind _as_bp_third_person_character_2 (Variables|Default|GetAs%20BP%20Third%20Person%20Character))
  (bind _hud2 (Variables|/Game/ThirdPerson/Blueprints/BP_ThirdPersonCharacter.BP_ThirdPersonCharacter_C|GetHUD2 _as_bp_third_person_character))
  ;[0 0 0] Changer réfs Player
  (Default|TimeFragments _as_bp_third_person_character)
  (Widget|SetVisibility _hud2 "Visible")
  (Variables|/Game/UI/Character_UI/WB_HUD2.WB_HUD2_C|SetAdd_Lucioles _hud2 (Variables|Default|GetLucioles_Given))
  (Default|LuciolesGot _hud2)
  (Variables|/Game/ThirdPerson/Blueprints/BP_ThirdPersonCharacter.BP_ThirdPersonCharacter_C|SetTimeFragmentsNb _as_bp_third_person_character_2 (+ (Variables|/Game/ThirdPerson/Blueprints/BP_ThirdPersonCharacter.BP_ThirdPersonCharacter_C|GetTimeFragmentsNb _as_bp_third_person_character_2) (Variables|Default|GetTime_Fragments_given)))
  (Default|TfGot _hud2))

(event Custom|Flower%20Destroyed
  (bind _as_bp_third_person_character (Variables|Default|GetAs%20BP%20Third%20Person%20Character))
  ;[0 0 0] Changer réfs Player
  ;;[0 1 0.1191] Flowers
  (bind _result (Math|Integer|IncrementInt (Variables|/Game/ThirdPerson/Blueprints/BP_ThirdPersonCharacter.BP_ThirdPersonCharacter_C|GetCorrupted_Flowers_Number _as_bp_third_person_character))
    (:%20%20
      (Variables|/Game/ThirdPerson/Blueprints/BP_ThirdPersonCharacter.BP_ThirdPersonCharacter_C|SetCorrupted_Flowers_Number _as_bp_third_person_character _result))))

(event Custom|Verify%20All%20flowers
  (bind _as_bp_third_person_character (Variables|Default|GetAs%20BP%20Third%20Person%20Character))
  ;[0 0 0] Changer réfs Player
  ;;[0 1 0.1191] Flowers
  (if (== (Variables|/Game/ThirdPerson/Blueprints/BP_ThirdPersonCharacter.BP_ThirdPersonCharacter_C|GetCorrupted_Flowers_Number _as_bp_third_person_character) (Variables|/Game/ThirdPerson/Blueprints/BP_ThirdPersonCharacter.BP_ThirdPersonCharacter_C|GetMax_Corrupted_Flowers_Number _as_bp_third_person_character))
    (Default|RelancementDeLaZone (Variables|Default|GetManager))
    (CallFunction|Rewards)))

(event EventBeginPlay
  (bind _sphere (Variables|Default|GetSphere))
  ;[0 0 0] Changer réfs Player
  (|CallParentFunction)
  (Utilities|FlowControl|Delay (Variables|Init|GetTime%20Before%20Growing))
  (Variables|Default|SetInitialScale (Transformation|GetWorldTransform _sphere))
  (Transformation|SetWorldTransform _sphere (Math|Transform|MakeTransform (.location (Variables|Default|GetInitialScale)) (.rotation (Variables|Default|GetInitialScale)) (* (.scale (Variables|Default|GetInitialScale)) (Variables|Init|GetNewScale))) false false))

(event EventInteraction
  ;[0 0 0] Changer réfs Player
  (Default|RelancementDeLaZone (Variables|Default|GetManager)))

(fn ConstructionScript
  (|CallParentFunction))