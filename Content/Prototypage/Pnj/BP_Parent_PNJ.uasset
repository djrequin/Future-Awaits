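; Parent NPC Blueprint that lets the player open a dialog and can update the game's goal.
; BeginPlay caches the game mode and player character and converts the character-name enums to strings.
; Interaction, gated by a resettable DoOnce, spawns WB_Dialog_System with the dialog lines, names and itself.
; ResetContents swaps in new dialog, optionally pushes a new goal to the game mode, then re-enables interaction.
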(event Custom|post_dialog)

(event Custom|Reset_Untalk
  (Utilities|FlowControl|DoOnce false) ; enters at Reset
)

(event Custom|Set_new_goal
  (Default|ChangeGoal (Variables|Default|GetAs%20BP%20Third%20Person%20Game%20Mode) (Variables|Default|GetNew%20goal%20) (Variables|Default|GetStatus)))

(event EventBeginPlay
  (bind _asbp_third_person_game_mode (Utilities|Casting|CastToBP_ThirdPersonGameMode (Game|GetGameMode)))
  (Variables|Default|SetAs%20BP%20Third%20Person%20Game%20Mode _asbp_third_person_game_mode)
  (bind _asbp_third_person_character (Utilities|Casting|CastToBP_ThirdPersonCharacter (Game|GetPlayerCharacter 0)))
  (Variables|Default|SetAs%20BP%20Third%20Person%20Character_0 _asbp_third_person_character)
  (Variables|Default|SetText%20to%20print (Variables|Default|GetName))
  (for _array_element (Variables|Default|GetCharacter_name)
    (Utilities|Array|Add (Variables|Default|GetNames_array) (Utilities|String|EnumtoString _array_element))))

(event EventDisplayName
  (params (Widget%20%28Tirer%20"show"%29 :type WB%20Interaction%20Button%20Object%20Reference))
  (Default|Show Widget%20%28Tirer%20"show"%29 (Variables|Default|GetText%20to%20print)))

(event EventInteraction
  (Utilities|FlowControl|DoOnce false
    (:Completed
      (bind _returnvalue (UserInterface|CreateWidget "/Game/UI/Character_UI/WB_Dialog_System.WB_Dialog_System_C"))
      (UserInterface|Viewport|AddtoViewport _returnvalue 0)
      (Default|Init _returnvalue (Variables|Default|GetDialogs) (Variables|Default|GetNames_array) self))))

(fn ConstructionScript)

(fn ResetContents
  (params (Content :type Array%20of%20Texts) (Names :type Array%20of%20Strings) (HasNewGoal :type Boolean) (Goal :type String) (Status :type Enum_Goal%20Enum :default "NewEnumerator0"))
  (Variables|Default|SetDialogs Content)
  (Variables|Default|SetNames_array Names)
  (Math|Integer|IncrementInt (Variables|Default|GetLine)
    (:%20%20
      (if HasNewGoal
        (Variables|Default|SetNew%20goal%20 Goal)
        (Variables|Default|SetStatus Status)
        (CallFunction|SetNewGoal))
      (CallFunction|ResetUntalk))))