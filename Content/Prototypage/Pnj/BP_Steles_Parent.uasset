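; Parent Blueprint for readable stele actors that show their text in a dialog when interacted with.
; On BeginPlay it converts its Titles enum values into a list of name strings.
; Interaction, gated by CanRead, clears that flag, then creates a WB_Dialog_System widget and initializes it with the text, names and a reference to itself.
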(event EventBeginPlay
  (|CallParentFunction)
  (for _array_element (Variables|Default|GetTitles)
    (Utilities|Array|Add (Variables|Default|GetNames) (Utilities|String|EnumtoString _array_element))))

(event Collision|EventActorBeginOverlap
  (params (OtherActor :type Actor%20Object%20Reference)))

(event EventTick
  (params (DeltaSeconds :type Float%20%28single-precision%29))
  (|CallParentFunction DeltaSeconds) ; This node is disabled and will not be called.\nDrag off pins to build functionality.
)

(event EventInteraction
  (if (Variables|Default|GetCanRead?)
    (Variables|Default|SetCanRead? false)
    (bind _returnvalue (UserInterface|CreateWidget "/Game/UI/Character_UI/WB_Dialog_System.WB_Dialog_System_C"))
    (UserInterface|Viewport|AddtoViewport _returnvalue 0)
    (Default|Init _returnvalue (Variables|Default|GetText) (Variables|Default|GetNames) 0 self)))

(fn ConstructionScript
  (|CallParentFunction))