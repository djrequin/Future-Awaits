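; BP_Dialog_Box is a trigger box that starts a dialogue, and optionally a cutscene, when the third-person character overlaps it.
; BeginPlay converts the speaker name enums to strings, and a one-shot overlap passes them with the lines, voices and timings to the character's DynamicUI.
; If it contains a cutscene, it blocks player movement and plays the level sequence, then restores movement and destroys itself when the sequence stops.
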(event OnComponentBeginOverlap(Box)
  (params (OverlappedComponent :type Primitive%20Component%20Object%20Reference) (OtherActor :type Actor%20Object%20Reference) (OtherComp :type Primitive%20Component%20Object%20Reference) (OtherBodyIndex :type Integer) (bFromSweep :type Boolean) (SweepResult :type Hit%20Result%20Structure%20%28by%20ref%29))
  (bind _asbp_third_person_character (Utilities|Casting|CastToBP_ThirdPersonCharacter OtherActor))
  (Utilities|FlowControl|DoOnce false
    (:Completed
      (Utilities|FlowControl|Sequence
        (:then_0
          ;[1 0 0.2603] Initialisation des dialogues
          (Default|Initialize (Variables|/Game/ThirdPerson/Blueprints/BP_ThirdPersonCharacter.BP_ThirdPersonCharacter_C|GetDynamic_UI _asbp_third_person_character) (Variables|Basics|GetDelays) (Variables|Basics|GetVoices) (Variables|Basics|GetContent) (Variables|Basics|GetNames_array) (Variables|Basics|GetLines_delay)))
        (:then_1
          ;[1 0.3844 0.6303] Gestion des cinématiques
          (if (Variables|Cutscene|GetContains_Cutscene?)
            (Default|CannotMove _asbp_third_person_character false)
            (bind (_outactor _returnvalue) (Sequencer|Player|CreateLevelSequencePlayer (Variables|Cutscene|GetCutscene_to_play)))
            (Sequencer|Player|Play (Variables|/Script/LevelSequence.LevelSequenceActor|GetSequencePlayer _outactor) :!class /Script/MovieScene.MovieSceneSequencePlayer)
            (EventDispatchers|BindEventtoOnStop _returnvalue (delegate Custom|move))))))))

(event Custom|move
  ;[1 0.3844 0.6303] Gestion des cinématiques
  (Default|CanMoveAgain (stale OnComponentBeginOverlap(Box) _asbp_third_person_character))
  (Actor|DestroyActor))

(event EventBeginPlay
  (for _array_element (Variables|Basics|GetCharacter_name)
    (Utilities|Array|Add (Variables|Basics|GetNames_array) (Utilities|String|EnumtoString _array_element))))

(fn ConstructionScript)