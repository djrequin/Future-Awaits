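; Ailem NPC Blueprint that reacts to the end of a dialogue by moving toward its current goal.
; PostDialog consumes the one-shot HasAPDGoal flag to call SetNewGoal, or prints a French "no new objective" debug message.
; It then sends the pawn via AIMoveTo to the location of the Goal entry indexed by Line, if valid.
; BeginPlay and the construction script add no logic of their own.
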(event EventBeginPlay
  (|CallParentFunction) ; This node is disabled and will not be called.\nDrag off pins to build functionality.
)

(event EventPostDialog
  (bind _goal (Variables|Default|GetGoal))
  (bind _line (Variables|Default|GetLine))
  (bind _output (Utilities|Array|Get(acopy) _goal _line))
  (if (Variables|Default|GetHas_a_PD_goal?)
    (Variables|Default|SetHas_a_PD_goal? false)
    (CallFunction|SetNewGoal)
    (else
      (Development|PrintString "Pas de nouvel objectif")))
  (Utilities|IsValid _output
    (:Is%20Valid
      (AI|AIMoveTo self (Transformation|GetWorldLocation (Variables|/Game/Prototypage/Pnj/BP_Goal_AI.BP_Goal_AI_C|GetDefaultSceneRoot _output)) 0 5.0 false))))

(fn ConstructionScript
  (|CallParentFunction))