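; End-game trigger that starts a new "Collecter les souvenirs" (collect the memories) goal when the BP_Ailem actor enters its box.
; On BeginPlay it registers itself as EndGame on BP_ThirdPersonGameMode and converts its enum name list into strings.
; On overlap it passes its content, names and new goal to Ailem through ResetContents, unhides Ailem, prints a debug message and flags itself as started.
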(event OnComponentBeginOverlap(Box)
  (params (OverlappedComponent :type Primitive%20Component%20Object%20Reference) (OtherActor :type Actor%20Object%20Reference) (OtherComp :type Primitive%20Component%20Object%20Reference) (OtherBodyIndex :type Integer) (bFromSweep :type Boolean) (SweepResult :type Hit%20Result%20Structure%20%28by%20ref%29))
  (bind _asbp_ailem (Utilities|Casting|CastToBP_Ailem OtherActor))
  (bind _output_get (Variables|Default|SetAs%20BP%20Ailem _asbp_ailem))
  (Development|PrintString "Ailem In" true true "(R=1.000000,G=0.058055,B=0.658764,A=1.000000)" 5.0)
  (Default|ResetContents _asbp_ailem (Variables|Default|GetContent) (Variables|Default|GetNames) true true "Collecter les souvenirs" "NewEnumerator3" 0 false false)
  (Rendering|SetActorHiddenInGame _output_get false)
  (Variables|Default|SetStarted true))

(event EventBeginPlay
  (bind _asbp_third_person_game_mode (Utilities|Casting|CastToBP_ThirdPersonGameMode (Game|GetGameMode)))
  (bind _output_get (Variables|Default|SetAs%20BP%20Third%20Person%20Game%20Mode _asbp_third_person_game_mode))
  (Variables|/Game/ThirdPerson/Blueprints/BP_ThirdPersonGameMode.BP_ThirdPersonGameMode_C|SetEnd_game _output_get self)
  (for _array_element (Variables|Default|GetNamess)
    (Utilities|Array|Add (Variables|Default|GetNames) (Utilities|String|EnumtoString _array_element))))

(fn ConstructionScript)