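; BP_Goal_AI is a one-shot trigger actor that updates the state of an NPC (BP_Parent_PNJ) that enters its box.
; On BeginPlay it converts its NewNames enum entries into a string array.
; On box overlap with such an NPC, it calls ResetContents to pass new content, names, goal settings, status and a linked corrupted flower, then destroys itself.
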(event OnComponentBeginOverlap(Box)
  (params (OverlappedComponent :type Primitive%20Component%20Object%20Reference) (OtherActor :type Actor%20Object%20Reference) (OtherComp :type Primitive%20Component%20Object%20Reference) (OtherBodyIndex :type Integer) (bFromSweep :type Boolean) (SweepResult :type Hit%20Result%20Structure%20%28by%20ref%29))
  (bind _asbp_parent_pnj (Utilities|Casting|CastToBP_Parent_PNJ OtherActor))
  (Default|ResetContents _asbp_parent_pnj (Variables|Dialogs|GetNew_content) (Variables|Dialogs|GetNames_array) (Variables|Goals|GetSet_new_Goal) (Variables|Goals|GetNew%20Goal%20post_dialog%20?) (Variables|Goals|GetNew_Goal) (Variables|Goals|GetStatus) (Variables|Default|GetCorrupted_Flower))
  (Actor|DestroyActor))

(event EventBeginPlay
  (for _array_element (Variables|Dialogs|GetNew%20names)
    (Utilities|Array|Add (Variables|Dialogs|GetNames_array) (Utilities|String|EnumtoString _array_element))))

(event Collision|EventActorBeginOverlap
  (params (OtherActor :type Actor%20Object%20Reference)))

(event EventTick
  (params (DeltaSeconds :type Float%20%28single-precision%29)))

(fn ConstructionScript)