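; Interactable chest that grants lucioles and time fragments to Melia once opened.
; Unless it starts openable, it is unlocked either by clearing an enemy camp or through linked threads, each destroying a vine with a blink effect.
; A looping Timeline polls the camp's enemy list for invalid entries to count kills.
; Locked chests start with zero custom time dilation, restored when rewards are given.
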(event Custom|Can%20Set%20Open%20?%20%28Threads%29
  (bind _lianes (Variables|Default|GetLianes))
  (bind _threads_number (Variables|Default|GetThreads%20number))
  (bind _returnvalue (- _threads_number 1))
  (bind _output (Utilities|Array|Get(acopy) _lianes _returnvalue))
  (Utilities|IsValid _output
    (:Is%20Valid
      (Niagara|SpawnSystematLocation "/Game/BlinkAndDashVFX/VFX_Niagara/NS_Blink_DarkMagic.NS_Blink_DarkMagic" (Transformation|GetWorldLocation _output)))
    (:Is%20Not%20Valid
      _))
  (Utilities|IsValid _output
    (:Is%20Valid
      (Components|DestroyComponent _output))
    (:Is%20Not%20Valid
      _))
  (if (== (Utilities|Array|Length (Variables|Threads|GetThreads)) (Variables|Default|GetThreads%20number))
    (Variables|Default|SetPrint_interacton true)
    (Variables|Default|SetCan_Be_Opened? true)))

(event Custom|Rewards
  (bind _as_bp_melia_0 (Variables|Default|GetAs%20BP%20Melia_0))
  (bind _as_bp_melia_0_2 (Variables|Default|GetAs%20BP%20Melia_0))
  (bind _hud2 (Variables|/Game/ThirdPerson/Blueprints/BP_Melia.BP_Melia_C|GetHUD2 _as_bp_melia_0_2))
  (Utilities|FlowControl|DoOnce false
    (:Completed
      (Audio|SpawnSound2D "/Game/Sounds/Chests/OBJECT_CHEST_OPEN.OBJECT_CHEST_OPEN" 1.0 1.0 0.0 0)
      (Variables|/Game/ThirdPerson/Blueprints/BP_Melia.BP_Melia_C|SetThreads_Number _as_bp_melia_0_2 0)
      (Default|TimeFragments _as_bp_melia_0_2)
      (Widget|SetVisibility _hud2 "Visible")
      (Variables|/Game/UI/Character_UI/WB_HUD2.WB_HUD2_C|SetAdd_Lucioles _hud2 (Variables|Default|GetLucioles_Given))
      (Default|LuciolesGot _hud2)
      (Variables|/Game/ThirdPerson/Blueprints/BP_Melia.BP_Melia_C|SetTimeFragmentsNb _as_bp_melia_0 (+ (Variables|/Game/ThirdPerson/Blueprints/BP_Melia.BP_Melia_C|GetTimeFragmentsNb _as_bp_melia_0) (Variables|Default|GetTime_Fragments_given)))
      (Default|TfGot _hud2)
      (Variables|Default|SetPrint_interacton false)
      (Default|Hide (Variables|Default|GetButton))
      (Variables|Default|SetCustomTimeDilation 1.0))))

(event Custom|Set%20open%20?%20%28Enemies%29
  (if (== (Variables|Default|GetEnnemies_max) (Variables|Ennemies|Getennemies_number))
    (Variables|Default|SetCan_Be_Opened? true)))

(event Custom|Ennemies_Verification
  (Utilities|FlowControl|DoOnce false
    (:Completed
      (if (Variables|Default|GetEnnemy%20camp?)
        (if (not (Variables|Default|GetCan_Be_Opened?)) :!label _label
          (for _array_element (Variables|Ennemies|GetEnnemies)
            (Utilities|IsValid _array_element
              (:Is%20Not%20Valid
                (bind _result (Math|Integer|IncrementInt (Variables|Ennemies|Getennemies_number))
                  (:%20%20
                    (Variables|Ennemies|Setennemies_number _result)
                    (Utilities|Array|RemoveItem (Variables|Ennemies|GetEnnemies) _array_element))))))
          (CallFunction|SetOpen?(Enemies))
          (Timeline|Timeline PlayFromStart
            (:Finished
              (goto _label))))))))

(event EventBeginPlay
  (|CallParentFunction)
  (bind _asbp_melia (Utilities|Casting|CastToBP_Melia (Game|GetPlayerCharacter 0)))
  (Variables|Default|SetAs%20BP%20Melia_0 _asbp_melia)
  (Variables|Default|SetEnnemies_max (Utilities|Array|Length (Variables|Ennemies|GetEnnemies)))
  (CallFunction|EnnemiesVerification)
  (Variables|Default|SetWas_opened? (Variables|Default|GetCan_Be_Opened?))
  (bind _asbp_third_person_game_mode (Utilities|Casting|CastToBP_ThirdPersonGameMode (Game|GetGameMode)))
  (Variables|Default|SetAs%20BP%20Third%20Person%20Game%20Mode _asbp_third_person_game_mode)
  (CallFunction|Init)
  (for _array_element (Variables|Threads|GetThreads)
    (Utilities|IsValid _array_element
      (:Is%20Valid
        (Variables|/Game/Prototypage/Collectibles/Chests/BP_Threads.BP_Threads_C|SetChest _array_element self))))
  (if (Variables|Default|GetCan_Be_Opened?)
    (Variables|Default|SetPrint_interacton true)
    (else
      (Variables|Default|SetCustomTimeDilation 0.0))))

(event Collision|EventActorBeginOverlap
  (params (OtherActor :type Actor%20Object%20Reference)))

(event EventInteraction
  (if (Variables|Default|GetCan_Be_Opened?)
    (Default|Tuto (Variables|Default|GetAs%20BP%20Third%20Person%20Game%20Mode) "NewEnumerator2")
    (CallFunction|Rewards)
    (elif (Variables|Default|GetEnnemy%20camp?)
      (CallFunction|SetOpen?(Enemies))
      (else
        (CallFunction|CanSetOpen?(Threads))))))

(fn ConstructionScript
  (|CallParentFunction))

(fn Init
  (Variables|Default|SetLianes (Utilities|Array|MakeArray (Variables|Default|GetLiane1) (Variables|Default|GetLiane2) (Variables|Default|GetLiane3)))
  (if (Variables|Default|GetCan_Be_Opened?)
    (for _array_element (Variables|Default|GetLianes)
      (Components|DestroyComponent _array_element)
      (Development|PrintString "Hello"))))