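; BP_Threads is a thread collectible, filed under chest collectibles, that the player cuts by shooting it or interacting with it.
; Both the ShotEvent and Interaction events call a shared Cut event.
; Cut increments ThreadsNumber on the BP_Melia reference, then destroys the thread actor.
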(event Custom|Cut
  (Math|Integer|IncrementInt (Variables|/Game/ThirdPerson/Blueprints/BP_Melia.BP_Melia_C|GetThreads_Number (Variables|Default|GetAs%20BP%20Melia))
    (:%20%20
      (Actor|DestroyActor))))

(event EventBeginPlay
  (|CallParentFunction))

(event EventTick
  (params (DeltaSeconds :type Float%20%28single-precision%29))
  (|CallParentFunction DeltaSeconds) ; This node is disabled and will not be called.\nDrag off pins to build functionality.
)

(event EventInteraction
  (CallFunction|Cut))

(event EventShotEvent
  (CallFunction|Cut))

(fn ConstructionScript
  (|CallParentFunction))