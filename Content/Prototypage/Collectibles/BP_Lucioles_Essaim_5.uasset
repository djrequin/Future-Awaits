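; BP_Lucioles_Essaim_5 is a collectible firefly swarm Blueprint worth five lucioles, built on a parent class.
; On BeginPlay it runs the parent logic, sets GivenLuciolesNumber to five, then calls AllSPheresShining.
; That event switches Sphere2 from a low-shine to a high-shine material using timed delays, running once without looping.
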(event Custom|AllSPheresShining
  (Utilities|FlowControl|Sequence
    (:then_0
      (Rendering|Material|SetMaterial (Variables|Default|GetSphere2) 0 "/Game/Prototypage/Materials/M_ShineLow.M_ShineLow")
      (Utilities|FlowControl|Delay 1.0)
      (Rendering|Material|SetMaterial (Variables|Default|GetSphere2) 0 "/Game/Prototypage/Materials/M_ShineHigh.M_ShineHigh")
      (Utilities|FlowControl|Delay 1.0))))

(event EventBeginPlay
  (|CallParentFunction)
  (Variables|Default|SetGiven_Lucioles_Number 5)
  (CallFunction|AllSPheresShining))

(event Collision|EventActorBeginOverlap
  (params (OtherActor :type Actor%20Object%20Reference)))

(event EventTick
  (params (DeltaSeconds :type Float%20%28single-precision%29)))

(fn ConstructionScript
  (|CallParentFunction))