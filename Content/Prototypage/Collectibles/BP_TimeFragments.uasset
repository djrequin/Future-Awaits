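; BP_TimeFragments is a Time Fragment collectible that the player character Melia picks up by interaction.
; The Interaction event increments Melia's fragment count, then, if her HUD2 widget is valid, shows it and calls TfGot.
; In that same valid-HUD branch it triggers a tutorial step on the third-person game mode and destroys itself, so without a HUD the pickup stays in the world.
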(event EventBeginPlay
  (|CallParentFunction) ; This node is disabled and will not be called.\nDrag off pins to build functionality.
)

(event EventTick
  (params (DeltaSeconds :type Float%20%28single-precision%29))
  (|CallParentFunction DeltaSeconds) ; This node is disabled and will not be called.\nDrag off pins to build functionality.
)

(event EventInteraction
  (bind _as_bp_melia (Variables|Default|GetAs%20BP%20Melia))
  (bind _hud2 (Variables|/Game/ThirdPerson/Blueprints/BP_Melia.BP_Melia_C|GetHUD2 _as_bp_melia))
  (Math|Float|IncrementFloat (Variables|/Game/ThirdPerson/Blueprints/BP_Melia.BP_Melia_C|GetTimeFragmentsNb _as_bp_melia)
    (:%20%20
      (Utilities|IsValid _hud2
        (:Is%20Valid
          (Widget|SetVisibility _hud2 "Visible")
          (Default|TfGot _hud2)
          (Default|Tuto (Variables|/Game/ThirdPerson/Blueprints/BP_Melia.BP_Melia_C|GetAs%20BP%20Third%20Person%20Game%20Mode (Variables|Default|GetAs%20BP%20Melia)) "NewEnumerator1")
          (Actor|DestroyActor))))))

(fn ConstructionScript
  (|CallParentFunction))