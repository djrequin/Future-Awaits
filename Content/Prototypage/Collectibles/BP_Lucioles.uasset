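; BP_Lucioles is a collectible that awards fireflies (lucioles) to BP_Melia when she overlaps its sphere.
; On pickup it shows the player's HUD2, passes it the given firefly count and triggers its LuciolesGot update.
; It also calls Tuto on the cached BP_ThirdPersonGameMode, spawns a scaled Lucioles particle system at its location, then destroys itself.
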(event OnComponentBeginOverlap(Sphere)
  (params (OverlappedComponent :type Primitive%20Component%20Object%20Reference) (OtherActor :type Actor%20Object%20Reference) (OtherComp :type Primitive%20Component%20Object%20Reference) (OtherBodyIndex :type Integer) (bFromSweep :type Boolean) (SweepResult :type Hit%20Result%20Structure%20%28by%20ref%29))
  (bind _asbp_melia (Utilities|Casting|CastToBP_Melia OtherActor))
  (Widget|SetVisibility (Variables|/Game/ThirdPerson/Blueprints/BP_Melia.BP_Melia_C|GetHUD2 _asbp_melia) "Visible")
  (Variables|/Game/UI/Character_UI/WB_HUD2.WB_HUD2_C|SetAdd_Lucioles (Variables|/Game/ThirdPerson/Blueprints/BP_Melia.BP_Melia_C|GetHUD2 _asbp_melia) (Variables|Default|GetGiven_Lucioles_Number))
  (Default|LuciolesGot (Variables|/Game/ThirdPerson/Blueprints/BP_Melia.BP_Melia_C|GetHUD2 _asbp_melia))
  (Default|Tuto (Variables|Default|GetAs%20BP%20Third%20Person%20Game%20Mode) "NewEnumerator0")
  (Niagara|SpawnSystematLocation "/Game/BlinkAndDashVFX/VFX_Niagara/Lucioles.Lucioles" (Transformation|GetActorLocation) "0, 0, 0" (Math|Conversions|ToVector(Float) (Variables|Default|GetNewVar)))
  (Actor|DestroyActor))

(event EventBeginPlay
  (bind _asbp_third_person_game_mode (Utilities|Casting|CastToBP_ThirdPersonGameMode (Game|GetGameMode)))
  (Variables|Default|SetAs%20BP%20Third%20Person%20Game%20Mode _asbp_third_person_game_mode))

(fn ConstructionScript)