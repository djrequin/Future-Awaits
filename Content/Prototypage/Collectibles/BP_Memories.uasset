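; BP_Memories is an interactable memory collectible with a bobbing sphere, driven by a timeline and FlipFlop.
; BeginPlay loads its dialog row from DT_DIalogs using the MemoryToGo enum and, for quest memories, converts Names to strings.
; Interaction shows a WB_Memory widget with that data.
; After a short delay, it increments Melia's MemoriesCollected, passes the count to the game mode's GameFinish and destroys itself.
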(event Custom|moving
  (Utilities|FlowControl|FlipFlop
    (:A
      (bind _newtrack_0 (Timeline|move PlayFromStart)
        (:Update
          (Transformation|SetRelativeLocation (Variables|Default|GetSphere) (Math|Vector|MakeVector 0.0 0.0 (Math|Float|Lerp 0.0 1e+01 _newtrack_0)) false false))
        (:Finished
          (CallFunction|Moving))))
    (:B
      (Timeline|move ReverseFromEnd))))

(event EventBeginPlay
  (|CallParentFunction)
  (Variables|Default|SetPrint_interacton true)
  (CallFunction|Moving)
  (CallFunction|ChooseDT)
  (bind _asbp_third_person_game_mode (Utilities|Casting|CastToBP_ThirdPersonGameMode (Game|GetGameMode)))
  (Variables|Default|SetAs%20BP%20Third%20Person%20Game%20Mode _asbp_third_person_game_mode)
  (if (Variables|Default|GetIn%20quest?)
    (for _array_element (Variables|Default|GetNames)
      (Utilities|Array|Add (Variables|Default|GetNames_array) (Utilities|String|EnumtoString _array_element)))))

(event EventInteraction
  (bind _returnvalue (UserInterface|CreateWidget "/Game/UI/Cutscenes_UI/WB_Memory.WB_Memory_C" 0 (Variables|Default|GetOut%20Row) (Variables|Default|GetContent) (Variables|Default|GetNames_array) (Variables|Default|GetIn%20quest?) (Variables|Default|GetAilem)))
  (UserInterface|Viewport|AddtoViewport _returnvalue 0)
  (Utilities|FlowControl|Delay 3.0)
  (bind _result (Math|Integer|IncrementInt (Variables|/Game/ThirdPerson/Blueprints/BP_Melia.BP_Melia_C|GetMemories_collected (Variables|Default|GetAs%20BP%20Melia)))
    (:%20%20
      (Default|GameFinish (Variables|Default|GetAs%20BP%20Third%20Person%20Game%20Mode) _result)
      (Actor|DestroyActor))))

(fn ConstructionScript
  (|CallParentFunction))

(fn ChooseDT
  (bind _returnvalue (Utilities|GetDataTableRow "/Game/UI/Cutscenes_UI/DT_DIalogs.DT_DIalogs" (Utilities|String|StringToName (Utilities|String|EnumtoString (Variables|Default|GetMemory_to_go))))
    (:then
      (Variables|Default|SetOut%20Row _returnvalue))))