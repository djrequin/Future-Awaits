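; Firefly (luciole) swarm Blueprint variant that sets its given firefly count to ten.
; On BeginPlay it runs the parent logic, sets that count, then calls the allotherspheres event.
; That event switches Sphere6 from a low-shine material to a high-shine one using timed delays, a single blink with no loop in this graph.
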(event Custom|allotherspheres
  (Utilities|FlowControl|Sequence
    (:then_0
      (Rendering|Material|SetMaterial (Variables|Default|GetSphere6) 0 "/Game/Prototypage/Materials/M_ShineLow.M_ShineLow")
      (Utilities|FlowControl|Delay 1.0)
      (Rendering|Material|SetMaterial (Variables|Default|GetSphere6) 0 "/Game/Prototypage/Materials/M_ShineHigh.M_ShineHigh")
      (Utilities|FlowControl|Delay 1.0))))

(event EventBeginPlay
  (|CallParentFunction)
  (Variables|Default|SetGiven_Lucioles_Number 10)
  (CallFunction|Allotherspheres))

(event Collision|EventActorBeginOverlap
  (params (OtherActor :type Actor%20Object%20Reference))
  (|CallParentFunction OtherActor) ; This node is disabled and will not be called.\nDrag off pins to build functionality.
)

(event EventTick
  (params (DeltaSeconds :type Float%20%28single-precision%29))
  (|CallParentFunction DeltaSeconds) ; This node is disabled and will not be called.\nDrag off pins to build functionality.
)

(fn ConstructionScript
  (|CallParentFunction))