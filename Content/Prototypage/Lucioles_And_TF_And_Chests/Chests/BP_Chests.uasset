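; Reward chest that, once unlocked, grants the player lucioles and time fragments one time through the TFLucioles UI and resets their thread count.
; Enemy-camp chests poll their enemy list on a looping Timeline, counting invalid references until the total matches the starting count.
; Other chests compare their Threads array length to the player's ThreadsNumber on interaction.
; Interacting with a locked chest only runs this check, so rewards need another interaction.
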(event Custom|Can%20Set%20Open%20?%20%28Threads%29
  (if (== (Utilities|Array|Length (Variables|Threads|GetThreads)) (Variables|/Game/ThirdPerson/Blueprints/BP_ThirdPersonCharacter.BP_ThirdPersonCharacter_C|GetThreads_Number (Variables|Default|GetAs%20BP%20Third%20Person%20Character)))
    (Variables|Default|SetCan_Be_Opened? true)))

(event Custom|Rewards
  (bind _as_bp_third_person_character (Variables|Default|GetAs%20BP%20Third%20Person%20Character))
  (bind _as_bp_third_person_character_2 (Variables|Default|GetAs%20BP%20Third%20Person%20Character))
  (bind _tf_lucioles (Variables|/Game/ThirdPerson/Blueprints/BP_ThirdPersonCharacter.BP_ThirdPersonCharacter_C|GetTF/Lucioles _as_bp_third_person_character_2))
  (Development|PrintString "Hello")
  (Utilities|FlowControl|DoOnce false
    (:Completed
      (Variables|/Game/ThirdPerson/Blueprints/BP_ThirdPersonCharacter.BP_ThirdPersonCharacter_C|SetThreads_Number _as_bp_third_person_character_2 0)
      (Default|TimeFragments _as_bp_third_person_character_2)
      (Widget|SetVisibility _tf_lucioles "Visible")
      (Variables|/Game/UI/Character_UI/WB_HUD2.WB_HUD2_C|SetAdd_Lucioles _tf_lucioles (Variables|Default|GetLucioles_Given))
      (Default|LuciolesGot _tf_lucioles)
      (Variables|/Game/ThirdPerson/Blueprints/BP_ThirdPersonCharacter.BP_ThirdPersonCharacter_C|SetTimeFragmentsNb _as_bp_third_person_character (+ (Variables|/Game/ThirdPerson/Blueprints/BP_ThirdPersonCharacter.BP_ThirdPersonCharacter_C|GetTimeFragmentsNb _as_bp_third_person_character) (Variables|Default|GetTime_Fragments_given)))
      (Default|TfGot _tf_lucioles))))

(event Custom|Set%20open%20?%20%28Enemies%29
  (if (== (Variables|Default|GetEnnemies_max) (Variables|Ennemies|Getennemies_number))
    (Variables|Default|SetCan_Be_Opened? true)))

(event Custom|Ennemies_Verification
  (Utilities|FlowControl|DoOnce false
    (:Completed
      (if (Variables|Default|GetEnnemy%20camp?)
        (if (not (Variables|Default|GetCan_Be_Opened?)) :!label _label
          (for _array_element (Variables|Ennemies|GetEnnemies)
            (Utilities|IsValid _array_element
              (:Is%20Not%20Valid
                (bind _result (Math|Integer|IncrementInt (Variables|Ennemies|Getennemies_number))
                  (:%20%20
                    (Variables|Ennemies|Setennemies_number _result)
                    (Utilities|Array|RemoveItem (Variables|Ennemies|GetEnnemies) _array_element)
                    (Development|PrintString "ggf"))))))
          (CallFunction|SetOpen?(Enemies))
          (Timeline|Timeline PlayFromStart
            (:Finished
              (goto _label))))))))

(event EventBeginPlay
  (|CallParentFunction)
  (bind _asbp_third_person_character (Utilities|Casting|CastToBP_ThirdPersonCharacter (Game|GetPlayerCharacter 0)))
  (Variables|Default|SetAs%20BP%20Third%20Person%20Character _asbp_third_person_character)
  (Variables|Default|SetEnnemies_max (Utilities|Array|Length (Variables|Ennemies|GetEnnemies)))
  (CallFunction|EnnemiesVerification))

(event Collision|EventActorBeginOverlap
  (params (OtherActor :type Actor%20Object%20Reference)))

(event EventInteraction
  (if (Variables|Default|GetCan_Be_Opened?)
    (CallFunction|Rewards)
    (elif (Variables|Default|GetEnnemy%20camp?)
      (CallFunction|SetOpen?(Enemies))
      (else
        (CallFunction|CanSetOpen?(Threads))))))

(event EventTick
  (params (DeltaSeconds :type Float%20%28single-precision%29)))

(fn ConstructionScript
  (|CallParentFunction))