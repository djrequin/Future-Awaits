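; BP_Threads is a thread actor that the player cuts by shooting or interacting with it, adding to their thread count.
; Both ShotEvent and Interaction route to a shared Cut event, which increments ThreadsNumber on the player character and destroys the actor.
; The BP_ThirdPersonCharacter reference is cast from player 0 and cached on BeginPlay.
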(event Custom|Cut
  (bind _as_bp_third_person_character (Variables|Default|GetAs%20BP%20Third%20Person%20Character))
  (bind _result (Math|Integer|IncrementInt (Variables|/Game/ThirdPerson/Blueprints/BP_ThirdPersonCharacter.BP_ThirdPersonCharacter_C|GetThreads_Number _as_bp_third_person_character))
    (:%20%20
      (Variables|/Game/ThirdPerson/Blueprints/BP_ThirdPersonCharacter.BP_ThirdPersonCharacter_C|SetThreads_Number _as_bp_third_person_character _result)
      (Actor|DestroyActor))))

(event EventBeginPlay
  (|CallParentFunction)
  (bind _asbp_third_person_character (Utilities|Casting|CastToBP_ThirdPersonCharacter (Game|GetPlayerCharacter 0)))
  (Variables|Default|SetAs%20BP%20Third%20Person%20Character _asbp_third_person_character))

(event EventTick
  (params (DeltaSeconds :type Float%20%28single-precision%29))
  (|CallParentFunction DeltaSeconds) ; This node is disabled and will not be called.\nDrag off pins to build functionality.
)

(event EventInteraction
  (CallFunction|Cut))

(event EventShotEvent
  (CallFunction|Cut))

(fn ConstructionScript
  (|CallParentFunction))