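; BP_Lucioles is a firefly pickup that adds to the player's lucioles count when touched.
; A self-recalling Shining event pulses the point light and swaps the sphere between low and high glow materials using delays.
; Overlap by the third-person character shows its HUD, passes it GivenLuciolesNumber, calls the game mode's Tuto, then destroys the actor.
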(event OnComponentBeginOverlap(Sphere)
  (params (OverlappedComponent :type Primitive%20Component%20Object%20Reference) (OtherActor :type Actor%20Object%20Reference) (OtherComp :type Primitive%20Component%20Object%20Reference) (OtherBodyIndex :type Integer) (bFromSweep :type Boolean) (SweepResult :type Hit%20Result%20Structure%20%28by%20ref%29))
  (bind _asbp_third_person_character (Utilities|Casting|CastToBP_ThirdPersonCharacter OtherActor))
  (Widget|SetVisibility (Variables|/Game/ThirdPerson/Blueprints/BP_ThirdPersonCharacter.BP_ThirdPersonCharacter_C|GetHUD2 _asbp_third_person_character) "Visible")
  (Variables|/Game/UI/Character_UI/WB_HUD2.WB_HUD2_C|SetAdd_Lucioles (Variables|/Game/ThirdPerson/Blueprints/BP_ThirdPersonCharacter.BP_ThirdPersonCharacter_C|GetHUD2 _asbp_third_person_character) (Variables|Default|GetGiven_Lucioles_Number))
  (Default|LuciolesGot (Variables|/Game/ThirdPerson/Blueprints/BP_ThirdPersonCharacter.BP_ThirdPersonCharacter_C|GetHUD2 _asbp_third_person_character))
  (Default|Tuto (Variables|Default|GetAs%20BP%20Third%20Person%20Game%20Mode) true)
  (Actor|DestroyActor))

(event Custom|Shining
  (Rendering|Material|SetMaterial (Variables|Default|GetSphere1) 0 "/Game/Prototypage/Materials/M_ShineLow.M_ShineLow")
  (Rendering|Components|Light|SetIntensity (Variables|Default|GetPointLight) 4e+03)
  (Utilities|FlowControl|Delay 1.0)
  (Rendering|Components|Light|SetIntensity (Variables|Default|GetPointLight) 7e+03)
  (Rendering|Material|SetMaterial (Variables|Default|GetSphere1) 0 "/Game/Prototypage/Materials/M_ShineHigh.M_ShineHigh")
  (Utilities|FlowControl|Delay 1.0)
  (CallFunction|Shining))

(event EventBeginPlay
  (CallFunction|Shining)
  (bind _asbp_third_person_game_mode (Utilities|Casting|CastToBP_ThirdPersonGameMode (Game|GetGameMode)))
  (Variables|Default|SetAs%20BP%20Third%20Person%20Game%20Mode _asbp_third_person_game_mode))

(fn ConstructionScript)