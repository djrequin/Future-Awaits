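; BP_TimeFragments is a collectible Time Fragment that the player picks up through its Interaction event.
; Interaction increments the fragment count on ThirdPersonCharacter, then, if the character's HUD2 is valid, shows it, calls TfGot and passes false to the game mode's Tuto.
; The actor destroys itself only on that valid-HUD branch, so without a HUD it still counts but stays in the world.
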(event EventBeginPlay
  (|CallParentFunction) ; This node is disabled and will not be called.\nDrag off pins to build functionality.
)

(event EventTick
  (params (DeltaSeconds :type Float%20%28single-precision%29))
  (|CallParentFunction DeltaSeconds) ; This node is disabled and will not be called.\nDrag off pins to build functionality.
)

(event EventInteraction
  (bind _thirdpersoncharacter (Variables|Default|GetThirdPersonCharacter))
  (bind _hud2 (Variables|/Game/ThirdPerson/Blueprints/BP_ThirdPersonCharacter.BP_ThirdPersonCharacter_C|GetHUD2 _thirdpersoncharacter))
  (Variables|/Game/ThirdPerson/Blueprints/BP_ThirdPersonCharacter.BP_ThirdPersonCharacter_C|SetTimeFragmentsNb _thirdpersoncharacter (+ (Variables|/Game/ThirdPerson/Blueprints/BP_ThirdPersonCharacter.BP_ThirdPersonCharacter_C|GetTimeFragmentsNb _thirdpersoncharacter) 1.0))
  (Utilities|IsValid _hud2
    (:Is%20Valid
      (Widget|SetVisibility _hud2 "Visible")
      (Default|TfGot _hud2)
      (Default|Tuto (Variables|/Game/ThirdPerson/Blueprints/BP_ThirdPersonCharacter.BP_ThirdPersonCharacter_C|GetAs%20BP%20Third%20Person%20Game%20Mode (Variables|Default|GetThirdPersonCharacter)) false)
      (Actor|DestroyActor))))

(fn ConstructionScript
  (|CallParentFunction))