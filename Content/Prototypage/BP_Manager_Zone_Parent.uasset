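; Parent zone manager that registers the frozen items, enemies, zone names and frozen zone managers inside its Box volume.
; After a delay on BeginPlay it scales up the Box, and overlaps fill its lists or hand frozen zone managers a back-reference before initializing them.
; The player character's current zone manager follows Box entry and exit.
; Relancementdelazone relaunches every registered frozen item and flags it frozen.
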(event OnComponentBeginOverlap(Box)
  (params (OverlappedComponent :type Primitive%20Component%20Object%20Reference) (OtherActor :type Actor%20Object%20Reference) (OtherComp :type Primitive%20Component%20Object%20Reference) (OtherBodyIndex :type Integer) (bFromSweep :type Boolean) (SweepResult :type Hit%20Result%20Structure%20%28by%20ref%29))
  (Utilities|FlowControl|Sequence
    (:then_0
      (bind _asbp_frozen_item_parent (Utilities|Casting|CastToBP_FrozenItemParent OtherActor))
      (bind _output_get (Variables|Default|SetAs%20Test%20Figer _asbp_frozen_item_parent))
      (Utilities|Array|Add (Variables|Default|GetfrozenItems) _output_get))
    (:then_1
      (bind _asbp_frozen_zone_manager (Utilities|Casting|CastToBP_Frozen_Zone_Manager OtherActor))
      (bind _output_get_2 (Variables|Default|SetAs%20Frozen_Zone _asbp_frozen_zone_manager))
      (Variables|/Game/Prototypage/Frozen_zone/BP_Frozen_Zone_Manager.BP_Frozen_Zone_Manager_C|SetManager _output_get_2 self)
      (Default|Initialisation _asbp_frozen_zone_manager))
    (:then_2
      (bind _asbp_ennemy_parent (Utilities|Casting|CastToBP_Ennemy_parent OtherActor))
      (Utilities|Array|Add (Variables|Default|GetEnnemis) _asbp_ennemy_parent))
    (:then_3
      (bind _asbp_third_person_character (Utilities|Casting|CastToBP_ThirdPersonCharacter OtherActor))
      (Variables|Default|SetAs%20BP%20Third%20Person%20Character _asbp_third_person_character)
      (Variables|/Game/ThirdPerson/Blueprints/BP_ThirdPersonCharacter.BP_ThirdPersonCharacter_C|SetCurrentZoneManager _asbp_third_person_character self))
    (:then_4
      (bind _asbp_zone_name (Utilities|Casting|CastToBP_Zone_Name OtherActor))
      (Utilities|Array|Add (Variables|Default|Getzone_names) _asbp_zone_name))))

(event OnComponentEndOverlap(Box)
  (params (OverlappedComponent :type Primitive%20Component%20Object%20Reference) (OtherActor :type Actor%20Object%20Reference) (OtherComp :type Primitive%20Component%20Object%20Reference) (OtherBodyIndex :type Integer))
  (bind _asbp_third_person_character (Utilities|Casting|CastToBP_ThirdPersonCharacter OtherActor))
  (Variables|/Game/ThirdPerson/Blueprints/BP_ThirdPersonCharacter.BP_ThirdPersonCharacter_C|SetCurrentZoneManager _asbp_third_person_character 0))

(event Custom|Relancement%20de%20la%20zone
  (for _array_element (Variables|Default|GetfrozenItems)
    (Default|Relancer _array_element)
    (Variables|/Game/Prototypage/Frozen_zone/BP_FrozenItemParent.BP_FrozenItemParent_C|SetIsFrozen? _array_element true)))

(event EventBeginPlay
  (bind _box (Variables|Default|GetBox))
  (Utilities|FlowControl|Delay (Variables|Default|GetTimeBeforeGrowing))
  (Variables|Default|SetInitialScale (Transformation|GetWorldTransform _box))
  (Transformation|SetWorldTransform _box (Math|Transform|MakeTransform (.location (Variables|Default|GetInitialScale)) (.rotation (Variables|Default|GetInitialScale)) (* (.scale (Variables|Default|GetInitialScale)) (Variables|Default|GetNewScale))) false false))

(fn ConstructionScript)