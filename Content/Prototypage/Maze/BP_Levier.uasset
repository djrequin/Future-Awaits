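; Maze lever that, on interaction, flips between two states, swapping which of two linked doors is open and which is closed.
; BeginPlay closes DoorToClose, then each interaction pitches the Sphere component up or down, toggles IsOpened and drives both doors in opposite directions.
; A DoOnce doubles both rotation deltas after the first pull, so later pulls swing twice as far.
; The interaction's own DoOnce resets immediately after each toggle.
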(event Custom|Increase_values
  (Utilities|FlowControl|DoOnce false
    (:Completed
      (Utilities|FlowControl|Sequence
        (:then_0
          (Variables|Default|SetDelta%20Rotation%20Y%20%28Bottom%29 (* (Variables|Default|GetDelta%20Rotation%20Y%20%28Bottom%29) 2.0)))
        (:then_1
          (Variables|Default|SetDelta%20Rotation%20Y%20%28Up%29 (* (Variables|Default|GetDelta%20Rotation%20Y%20%28Up%29) 2.0)))))))

(event Custom|reset%20do%20once
  (Utilities|FlowControl|DoOnce false) ; enters at Reset
)

(event Custom|Close_door
  (Default|Open (Variables|Default|GetDoor_to_open))
  (Default|Close (Variables|Default|GetDoor_to_close)))

(event Custom|Open_door
  (Default|Close (Variables|Default|GetDoor_to_open))
  (Default|Open (Variables|Default|GetDoor_to_close)))

(event EventBeginPlay
  (|CallParentFunction)
  (Default|Close (Variables|Default|GetDoor_to_close)))

(event EventInteraction
  (Utilities|FlowControl|DoOnce false
    (:Completed
      (if (Variables|Default|GetIs_opened?)
        (Transformation|AddWorldRotation (Variables|Default|GetSphere) (Math|Rotator|MakeRotator 0.0 (Variables|Default|GetDelta%20Rotation%20Y%20%28Up%29) 0.0) false false)
        (CallFunction|IncreaseValues)
        (Variables|Default|SetIs_opened? false)
        (CallFunction|CloseDoor)
        (else
          (Transformation|AddWorldRotation (Variables|Default|GetSphere) (Math|Rotator|MakeRotator 0.0 (Variables|Default|GetDelta%20Rotation%20Y%20%28Bottom%29) 0.0) false false)
          (CallFunction|IncreaseValues)
          (Variables|Default|SetIs_opened? true)
          (CallFunction|OpenDoor)))
      (CallFunction|ResetDoOnce))))

(fn ConstructionScript
  (|CallParentFunction))