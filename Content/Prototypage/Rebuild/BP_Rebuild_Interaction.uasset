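; Rebuild interaction that spends the player's Lucioles (fireflies) to replace a destroyed object.
; BeginPlay formats BuildCost as the parenthesised TextToPrint label.
; Interaction checks the balance, deducts the cost, then switches on ConstructionType to spawn a replacement at DestroyedObject's transform, destroying that object and itself.
; Only Mur and Escaliers spawn their own wall and stairs Blueprints; Porte, Pont and Tronc all spawn BP_Lucioles.
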(event Custom|Take%20Money
  (bind _thirdpersoncharacter (Variables|Default|GetThirdPersonCharacter))
  (Variables|/Game/ThirdPerson/Blueprints/BP_ThirdPersonCharacter.BP_ThirdPersonCharacter_C|SetLuciolesNumber _thirdpersoncharacter (- (Variables|/Game/ThirdPerson/Blueprints/BP_ThirdPersonCharacter.BP_ThirdPersonCharacter_C|GetLuciolesNumber _thirdpersoncharacter) (Variables|Default|GetBuild_Cost))))

(event EventBeginPlay
  (|CallParentFunction)
  (Variables|Default|SetText%20to%20print (Utilities|Text|ToText(String) (Utilities|String|Append "(" (Utilities|String|ToString(Integer) (Variables|Default|GetBuild_Cost)) ")"))))

(event EventTick
  (params (DeltaSeconds :type Float%20%28single-precision%29))
  (|CallParentFunction DeltaSeconds) ; This node is disabled and will not be called.\nDrag off pins to build functionality.
)

(event EventInteraction
  (bind _destroyed_object (Variables|Default|GetDestroyed_Object))
  (bind _destroyed_object_2 (Variables|Default|GetDestroyed_Object))
  (bind _destroyed_object_3 (Variables|Default|GetDestroyed_Object))
  (bind _destroyed_object_4 (Variables|Default|GetDestroyed_Object))
  (bind _destroyed_object_5 (Variables|Default|GetDestroyed_Object))
  (if (>= (Variables|/Game/ThirdPerson/Blueprints/BP_ThirdPersonCharacter.BP_ThirdPersonCharacter_C|GetLuciolesNumber (Variables|Default|GetThirdPersonCharacter)) (Variables|Default|GetBuild_Cost))
    (switch Utilities|FlowControl|Switch|SwitchonEnum_rebuild (Variables|Default|GetConstruction_type)
      (:NewEnumerator0
        (CallFunction|TakeMoney)
        (Game|SpawnActorfromClass "/Game/Prototypage/Collectibles/BP_Lucioles.BP_Lucioles_C" (Transformation|GetWorldTransform (Variables|/Game/Prototypage/Rebuild/BP_Rebuild_Object_Parent.BP_Rebuild_Object_Parent_C|GetDefaultSceneRoot _destroyed_object_4)) "Undefined" "MultiplyWithRoot" 0 0)
        (Actor|DestroyActor _destroyed_object_4)
        (Actor|DestroyActor))
      (:NewEnumerator1
        (CallFunction|TakeMoney)
        (Game|SpawnActorfromClass "/Game/Prototypage/Collectibles/BP_Lucioles.BP_Lucioles_C" (Transformation|GetWorldTransform (Variables|/Game/Prototypage/Rebuild/BP_Rebuild_Object_Parent.BP_Rebuild_Object_Parent_C|GetDefaultSceneRoot _destroyed_object_5)) "Undefined" "MultiplyWithRoot" 0 0)
        (Actor|DestroyActor _destroyed_object_5)
        (Actor|DestroyActor))
      (:NewEnumerator2
        (CallFunction|TakeMoney)
        (Game|SpawnActorfromClass "/Game/Prototypage/Collectibles/BP_Lucioles.BP_Lucioles_C" (Transformation|GetWorldTransform (Variables|/Game/Prototypage/Rebuild/BP_Rebuild_Object_Parent.BP_Rebuild_Object_Parent_C|GetDefaultSceneRoot _destroyed_object_2)) "Undefined" "MultiplyWithRoot" 0 0)
        (Actor|DestroyActor _destroyed_object_2)
        (Actor|DestroyActor))
      (:NewEnumerator3
        (CallFunction|TakeMoney)
        (Game|SpawnActorfromClass "/Game/Prototypage/Rebuild/BP_Wall.BP_Wall_C" (Transformation|GetWorldTransform (Variables|/Game/Prototypage/Rebuild/BP_Rebuild_Object_Parent.BP_Rebuild_Object_Parent_C|GetDefaultSceneRoot _destroyed_object_3)) "Undefined" "MultiplyWithRoot" 0 0)
        (Actor|DestroyActor _destroyed_object_3)
        (Actor|DestroyActor))
      (:NewEnumerator4
        (CallFunction|TakeMoney)
        (Game|SpawnActorfromClass "/Game/Prototypage/Rebuild/BP_Stairs.BP_Stairs_C" (Transformation|GetWorldTransform (Variables|/Game/Prototypage/Rebuild/BP_Rebuild_Object_Parent.BP_Rebuild_Object_Parent_C|GetDefaultSceneRoot _destroyed_object)) "Undefined" "MultiplyWithRoot" 0 0)
        (Actor|DestroyActor _destroyed_object)
        (Actor|DestroyActor)))
    (Development|PrintString "J'ai pas l'asset")))

(fn ConstructionScript
  (|CallParentFunction))