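; BP_Vision is an interactable that shows a vision on screen as a UI overlay.
; Its Interaction event passes through a DoOnce, so the vision triggers only on the first interaction.
; It then creates a WB_Vision widget, hands it the Lines text and ImagesVision images, and adds it to the viewport.
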(event EventBeginPlay
  (|CallParentFunction) ; This node is disabled and will not be called.\nDrag off pins to build functionality.
)

(event Collision|EventActorBeginOverlap
  (params (OtherActor :type Actor%20Object%20Reference)))

(event EventTick
  (params (DeltaSeconds :type Float%20%28single-precision%29)))

(event EventInteraction
  (Utilities|FlowControl|DoOnce false
    (:Completed
      (bind _returnvalue (UserInterface|CreateWidget "/Game/Prototypage/Visions_Melia/WB_Vision.WB_Vision_C"))
      (Variables|/Game/Prototypage/Visions_Melia/WB_Vision.WB_Vision_C|Settext _returnvalue (Variables|Default|GetLines))
      (Variables|/Game/Prototypage/Visions_Melia/WB_Vision.WB_Vision_C|SetImages_to_show _returnvalue (Variables|Default|GetImages_vision))
      (UserInterface|Viewport|AddtoViewport _returnvalue 0))))

(fn ConstructionScript
  (|CallParentFunction))