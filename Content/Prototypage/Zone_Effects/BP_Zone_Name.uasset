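; BP_Zone_Name is a one-shot trigger that displays a zone name on screen when BP_Melia enters its Box.
; The overlap creates a New_Zone_Name widget, passes it the ZoneName, starts FadeCreate, adds it to the viewport, then destroys the actor.
; IsSecretZone selects the widget's secret or base text color, with the secondary secret color made opaque for secret zones and fully transparent otherwise.
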(event OnComponentBeginOverlap(Box)
  (params (OverlappedComponent :type Primitive%20Component%20Object%20Reference) (OtherActor :type Actor%20Object%20Reference) (OtherComp :type Primitive%20Component%20Object%20Reference) (OtherBodyIndex :type Integer) (bFromSweep :type Boolean) (SweepResult :type Hit%20Result%20Structure%20%28by%20ref%29))
  (Utilities|Casting|CastToBP_Melia OtherActor)
  (Utilities|FlowControl|DoOnce false
    (:Completed
      (bind _returnvalue (UserInterface|CreateWidget "/Game/UI/Environment/New_Zone_Name.New_Zone_Name_C"))
      (Variables|Default|SetWidget _returnvalue)
      (if (Variables|Default|GetIs%20secret%20zone?)
        (Variables|/Game/UI/Environment/New_Zone_Name.New_Zone_Name_C|SetSecret%20color_text_2 (Variables|Default|GetWidget) (Utilities|Struct|MakeSlateColor (Utilities|Struct|MakeLinearColor (.r (.specifiedcolor (Variables|/Game/UI/Environment/New_Zone_Name.New_Zone_Name_C|GetSecret%20color (Variables|Default|GetWidget)))) (.g (.specifiedcolor (Variables|/Game/UI/Environment/New_Zone_Name.New_Zone_Name_C|GetSecret%20color (Variables|Default|GetWidget)))) (.b (.specifiedcolor (Variables|/Game/UI/Environment/New_Zone_Name.New_Zone_Name_C|GetSecret%20color (Variables|Default|GetWidget)))) 1.0) "UseColor_Specified"))
        (Variables|/Game/UI/Environment/New_Zone_Name.New_Zone_Name_C|SetText_color (Variables|Default|GetWidget) (Variables|/Game/UI/Environment/New_Zone_Name.New_Zone_Name_C|GetSecret%20color (Variables|Default|GetWidget)))
        (Variables|/Game/UI/Environment/New_Zone_Name.New_Zone_Name_C|SetZone_Name (Variables|Default|GetWidget) (Variables|Default|GetZone_Name))
        (Default|FadeCreate (Variables|Default|GetWidget))
        (UserInterface|Viewport|AddtoViewport (Variables|Default|GetWidget) 0)
        (Actor|DestroyActor)
        (else
          (Variables|/Game/UI/Environment/New_Zone_Name.New_Zone_Name_C|SetSecret%20color_text_2 (Variables|Default|GetWidget) (Utilities|Struct|MakeSlateColor (Utilities|Struct|MakeLinearColor 1.0 0.0 1.0 0.0) "UseColor_Specified"))
          (Variables|/Game/UI/Environment/New_Zone_Name.New_Zone_Name_C|SetText_color (Variables|Default|GetWidget) (Variables|/Game/UI/Environment/New_Zone_Name.New_Zone_Name_C|GetBase%20color (Variables|Default|GetWidget)))
          (Variables|/Game/UI/Environment/New_Zone_Name.New_Zone_Name_C|SetZone_Name (Variables|Default|GetWidget) (Variables|Default|GetZone_Name))
          (Default|FadeCreate (Variables|Default|GetWidget))
          (UserInterface|Viewport|AddtoViewport (Variables|Default|GetWidget) 0)
          (Actor|DestroyActor))))))

(event EventBeginPlay)

(event Collision|EventActorBeginOverlap
  (params (OtherActor :type Actor%20Object%20Reference)))

(event EventTick
  (params (DeltaSeconds :type Float%20%28single-precision%29)))

(fn ConstructionScript)