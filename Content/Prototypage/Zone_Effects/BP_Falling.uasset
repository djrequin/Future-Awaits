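; BP_Falling is a zone trigger that returns Melia to a checkpoint when she falls into it fast enough.
; On box overlap it checks that she is falling and that her downward speed meets MinimumFallVelocity, otherwise printing the speed if too slow.
; A qualifying fall adds a fade widget, then after a short delay teleports her capsule to the referenced Checkpoint, occasionally showing a warning dialogue from Ailem.
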(event OnComponentBeginOverlap(Box)
  (params (OverlappedComponent :type Primitive%20Component%20Object%20Reference) (OtherActor :type Actor%20Object%20Reference) (OtherComp :type Primitive%20Component%20Object%20Reference) (OtherBodyIndex :type Integer) (bFromSweep :type Boolean) (SweepResult :type Hit%20Result%20Structure%20%28by%20ref%29))
  (bind _asbp_melia (Utilities|Casting|CastToBP_Melia OtherActor))
  (Variables|Default|SetAs%20BP%20Melia _asbp_melia)
  (if (AI|Components|NavMovement|IsFalling (Variables|/Script/Engine.Character|GetCharacterMovement _asbp_melia))
    (if (>= (* (.z (Transformation|GetVelocity _asbp_melia)) -1.0) (Variables|Default|GetMinimum%20fall%20velocity))
      (Utilities|FlowControl|Sequence
        (:then_0
          (bind _returnvalue (UserInterface|CreateWidget "/Game/UI/Character_UI/Wb_Fade.Wb_Fade_C"))
          (UserInterface|Viewport|AddtoViewport _returnvalue 0))
        (:then_1
          (Utilities|FlowControl|Delay 0.5)
          (Transformation|SetWorldLocation (Variables|/Script/Engine.Character|GetCapsuleComponent (Variables|Default|GetAs%20BP%20Melia)) (Transformation|GetWorldLocation (Variables|/Game/Prototypage/Zone_Effects/BP_CheckPoint.BP_CheckPoint_C|GetDefaultSceneRoot (Variables|Default|GetCheckpoint))) false true)
          (if (== (Math|Random|RandomIntegerinRange 0 4) 2)
            (Default|Initialize (Variables|/Game/ThirdPerson/Blueprints/BP_Melia.BP_Melia_C|GetDynamic_UI (Variables|Default|GetAs%20BP%20Melia)) (Utilities|Array|MakeArray 3.0) 0 (Utilities|Array|MakeArray "Prends garde à ne pas tomber, Melia") (Utilities|Array|MakeArray "Ailem")))))
      (else
        (Development|PrintString (Utilities|String|ToString(Float) (* (.z (Transformation|GetVelocity _asbp_melia)) -1.0)))))))

(event EventBeginPlay)

(event Collision|EventActorBeginOverlap
  (params (OtherActor :type Actor%20Object%20Reference)))

(event EventTick
  (params (DeltaSeconds :type Float%20%28single-precision%29)))

(fn ConstructionScript)