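; BP_Water_Zone is a zone effect actor that changes BP_Melia's movement speed inside its box, presumably to simulate water.
; On overlap, it saves Melia's RunSpeed and sets MaxWalkSpeed to NewWalkSpeed behind a DoOnce with no reset, so only the first entry takes effect.
; Leaving the box writes the saved speed back to both MaxWalkSpeed and RunSpeed.
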(event OnComponentBeginOverlap(Box)
  (params (OverlappedComponent :type Primitive%20Component%20Object%20Reference) (OtherActor :type Actor%20Object%20Reference) (OtherComp :type Primitive%20Component%20Object%20Reference) (OtherBodyIndex :type Integer) (bFromSweep :type Boolean) (SweepResult :type Hit%20Result%20Structure%20%28by%20ref%29))
  (bind _asbp_melia (Utilities|Casting|CastToBP_Melia OtherActor))
  (Utilities|FlowControl|DoOnce false
    (:Completed
      (Variables|Default|SetInitial_Walk_Speed (Variables|/Game/ThirdPerson/Blueprints/BP_Melia.BP_Melia_C|GetRun%20speed _asbp_melia))
      (Variables|/Script/Engine.CharacterMovementComponent|SetMaxWalkSpeed (Variables|/Script/Engine.Character|GetCharacterMovement _asbp_melia) (Variables|Default|GetNew_Walk_Speed)))))

(event OnComponentEndOverlap(Box)
  (params (OverlappedComponent :type Primitive%20Component%20Object%20Reference) (OtherActor :type Actor%20Object%20Reference) (OtherComp :type Primitive%20Component%20Object%20Reference) (OtherBodyIndex :type Integer))
  (bind _asbp_melia (Utilities|Casting|CastToBP_Melia OtherActor))
  (Variables|/Script/Engine.CharacterMovementComponent|SetMaxWalkSpeed (Variables|/Script/Engine.Character|GetCharacterMovement _asbp_melia) (Variables|Default|GetInitial_Walk_Speed))
  (Variables|/Game/ThirdPerson/Blueprints/BP_Melia.BP_Melia_C|SetRun%20speed _asbp_melia (Variables|Default|GetInitial_Walk_Speed)))

(event EventBeginPlay)

(event Collision|EventActorBeginOverlap
  (params (OtherActor :type Actor%20Object%20Reference)))

(event EventTick
  (params (DeltaSeconds :type Float%20%28single-precision%29)))

(fn ConstructionScript)