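; BP_Corrupted_cloud_Zone is a corrupted cloud area that alters BP_Melia's walk speed and drains her mana while she is inside.
; Box overlap saves her run speed, applies the zone's speed, and starts StealMana, a delay loop that subtracts clamped mana, refreshes the HUD and reapplies the speed each tick.
; Leaving clears the loop's flag, restores her speed and calls her automatic mana regeneration.
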(event OnComponentBeginOverlap(Box)
  (params (OverlappedComponent :type Primitive%20Component%20Object%20Reference) (OtherActor :type Actor%20Object%20Reference) (OtherComp :type Primitive%20Component%20Object%20Reference) (OtherBodyIndex :type Integer) (bFromSweep :type Boolean) (SweepResult :type Hit%20Result%20Structure%20%28by%20ref%29))
  (bind _asbp_melia (Utilities|Casting|CastToBP_Melia OtherActor))
  (Development|PrintString "Hello")
  (Variables|Default|SetInitial_Walk_Speed (Variables|/Game/ThirdPerson/Blueprints/BP_Melia.BP_Melia_C|GetRun%20speed _asbp_melia))
  (Variables|/Script/Engine.CharacterMovementComponent|SetMaxWalkSpeed (Variables|/Script/Engine.Character|GetCharacterMovement _asbp_melia) (Variables|Default|GetNew_Walk_Speed))
  (Variables|/Game/ThirdPerson/Blueprints/BP_Melia.BP_Melia_C|SetNotSteal%20Mana? _asbp_melia false)
  (Variables|Default|SetGonna%20Die%20? true)
  (CallFunction|StealMana))

(event OnComponentEndOverlap(Box)
  (params (OverlappedComponent :type Primitive%20Component%20Object%20Reference) (OtherActor :type Actor%20Object%20Reference) (OtherComp :type Primitive%20Component%20Object%20Reference) (OtherBodyIndex :type Integer))
  (bind _asbp_melia (Utilities|Casting|CastToBP_Melia OtherActor))
  (Variables|/Script/Engine.CharacterMovementComponent|SetMaxWalkSpeed (Variables|/Script/Engine.Character|GetCharacterMovement _asbp_melia) (Variables|Default|GetInitial_Walk_Speed))
  (Variables|/Game/ThirdPerson/Blueprints/BP_Melia.BP_Melia_C|SetRun%20speed _asbp_melia (Variables|Default|GetInitial_Walk_Speed))
  (Variables|/Game/ThirdPerson/Blueprints/BP_Melia.BP_Melia_C|SetNotSteal%20Mana? _asbp_melia true)
  (Variables|Default|SetGonna%20Die%20? false)
  (if (<= (Variables|/Game/ThirdPerson/Blueprints/BP_Melia.BP_Melia_C|GetMagie%28PM%29 _asbp_melia) 0.0)
    (Variables|/Game/ThirdPerson/Blueprints/BP_Melia.BP_Melia_C|SetMagie%28PM%29 _asbp_melia 0.0))
  (Default|Auto-RegenMana _asbp_melia))

(event Custom|Steal%20Mana
  (bind _asbp_melia (Utilities|Casting|CastToBP_Melia (Game|GetPlayerCharacter 0)))
  (Variables|Default|SetAs%20BP%20Melia _asbp_melia)
  (if (Variables|Default|GetGonna%20Die%20?) :!label _label
    (Variables|/Game/ThirdPerson/Blueprints/BP_Melia.BP_Melia_C|SetNotSteal%20Mana? (Variables|Default|GetAs%20BP%20Melia) false)
    (Variables|/Game/ThirdPerson/Blueprints/BP_Melia.BP_Melia_C|SetMagie%28PM%29 (Variables|Default|GetAs%20BP%20Melia) (Math|Float|Clamp(Float) (- (Variables|/Game/ThirdPerson/Blueprints/BP_Melia.BP_Melia_C|GetMagie%28PM%29 (Variables|Default|GetAs%20BP%20Melia)) (Variables|Default|GetStolen%20Mana%20%28tick%29)) 0.0 (Variables|/Game/ThirdPerson/Blueprints/BP_Melia.BP_Melia_C|GetMagieMax (Variables|Default|GetAs%20BP%20Melia))))
    (Default|ShowHud (Variables|Default|GetAs%20BP%20Melia))
    (Default|ModifyWalkSpeed (Variables|Default|GetAs%20BP%20Melia) (Variables|Default|GetNew_Walk_Speed))
    (Utilities|FlowControl|Delay (Variables|Default|GetDelay_Between_Ticks))
    (goto _label)))

(event EventBeginPlay)

(event Collision|EventActorBeginOverlap
  (params (OtherActor :type Actor%20Object%20Reference)))

(event EventTick
  (params (DeltaSeconds :type Float%20%28single-precision%29)))

(fn ConstructionScript)