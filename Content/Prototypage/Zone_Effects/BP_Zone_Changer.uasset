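; BP_Zone_Changer is a trigger actor that opens LevelToGo when the player character enters its box and is allowed to change zone.
; IsEndZone selects the forward or backward exit, each checking its own permission flag on the character.
; Both set PreviousZone on the game instance and save all data before loading.
; The forward exit also saves the Sphere's location and rotation as previous position, then delays briefly before opening the level.
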(event OnComponentBeginOverlap(Box)
  (params (OverlappedComponent :type Primitive%20Component%20Object%20Reference) (OtherActor :type Actor%20Object%20Reference) (OtherComp :type Primitive%20Component%20Object%20Reference) (OtherBodyIndex :type Integer) (bFromSweep :type Boolean) (SweepResult :type Hit%20Result%20Structure%20%28by%20ref%29))
  (bind _sphere (Variables|Default|GetSphere))
  (bind _as_game_instance_future_awaits (Variables|Default|GetAs%20Game%20Instance%20Future%20Awaits))
  (bind _returnvalue (Transformation|GetWorldTransform _sphere))
  ;[1 1 1] Changer ref player
  (bind _asbp_third_person_character (Utilities|Casting|CastToBP_ThirdPersonCharacter OtherActor))
  (Variables|Default|SetAs%20BP%20Third%20Person%20Character _asbp_third_person_character)
  (if (Variables|Default|GetIsEndZone)
    (if (Variables|/Game/ThirdPerson/Blueprints/BP_ThirdPersonCharacter.BP_ThirdPersonCharacter_C|GetCanGoToNextZone? (Variables|Default|GetAs%20BP%20Third%20Person%20Character))
      (Variables|/Game/ThirdPerson/Blueprints/Game_Instance_Future_Awaits.Game_Instance_Future_Awaits_C|SetPrevious_Zone? _as_game_instance_future_awaits false)
      (Default|SaveAllDatas _as_game_instance_future_awaits)
      (Default|SavePreviousPosition _as_game_instance_future_awaits (Math|Transform|MakeTransform (.location _returnvalue) (.rotation _returnvalue) "1.000000,1.000000,1.000000"))
      (Utilities|FlowControl|Delay 0.2)
      (Game|OpenLevel(byObjectReference) (Variables|Default|GetLevel_to_go)))
    (elif (Variables|/Game/ThirdPerson/Blueprints/BP_ThirdPersonCharacter.BP_ThirdPersonCharacter_C|GetCan_Go_Previous_Zone? (Variables|Default|GetAs%20BP%20Third%20Person%20Character))
      (Variables|/Game/ThirdPerson/Blueprints/Game_Instance_Future_Awaits.Game_Instance_Future_Awaits_C|SetPrevious_Zone? _as_game_instance_future_awaits true)
      (Default|SaveAllDatas _as_game_instance_future_awaits)
      (Game|OpenLevel(byObjectReference) (Variables|Default|GetLevel_to_go)))))

(event EventBeginPlay
  (bind _asgame_instance_future_awaits (Utilities|Casting|CastToGame_Instance_Future_Awaits (Game|GetGameInstance)))
  (Variables|Default|SetAs%20Game%20Instance%20Future%20Awaits _asgame_instance_future_awaits))

(fn ConstructionScript)