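; Corrupted water zone that slows the player character and kills Melia if still inside after a delay.
; Box overlap lowers walk speed and a looping timer reapplies it; leaving restores the saved speed and clears the timer.
; StealMana runs a delayed, DoOnce-guarded loop that, despite its name, sets HP to zero, updates the HUD and calls CoupDuDestin.
; The gradual StolenHp subtraction is left unused.
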(event OnComponentBeginOverlap(Box)
  (params (OverlappedComponent :type Primitive%20Component%20Object%20Reference) (OtherActor :type Actor%20Object%20Reference) (OtherComp :type Primitive%20Component%20Object%20Reference) (OtherBodyIndex :type Integer) (bFromSweep :type Boolean) (SweepResult :type Hit%20Result%20Structure%20%28by%20ref%29))
  (bind _asbp_third_person_character (Utilities|Casting|CastToBP_ThirdPersonCharacter OtherActor))
  (Variables|Default|SetInitial_Walk_Speed (Variables|/Game/ThirdPerson/Blueprints/BP_ThirdPersonCharacter.BP_ThirdPersonCharacter_C|GetRun%20speed _asbp_third_person_character))
  (bind _returnvalue (Utilities|Time|SetTimerbyEvent (delegate Custom|Set%20speed) 0.1 true))
  (Variables|Default|SetTimer _returnvalue)
  (Variables|/Script/Engine.CharacterMovementComponent|SetMaxWalkSpeed (Variables|/Script/Engine.Character|GetCharacterMovement _asbp_third_person_character) (Variables|Default|GetNew_Walk_Speed))
  (Variables|Default|SetStart/stop true)
  (Variables|/Game/ThirdPerson/Blueprints/BP_ThirdPersonCharacter.BP_ThirdPersonCharacter_C|SetNotSteal%20Mana? _asbp_third_person_character false)
  (CallFunction|StealMana))

(event OnComponentEndOverlap(Box)
  (params (OverlappedComponent :type Primitive%20Component%20Object%20Reference) (OtherActor :type Actor%20Object%20Reference) (OtherComp :type Primitive%20Component%20Object%20Reference) (OtherBodyIndex :type Integer))
  (bind _asbp_third_person_character (Utilities|Casting|CastToBP_ThirdPersonCharacter OtherActor))
  (Variables|/Script/Engine.CharacterMovementComponent|SetMaxWalkSpeed (Variables|/Script/Engine.Character|GetCharacterMovement _asbp_third_person_character) (Variables|Default|GetInitial_Walk_Speed))
  (Variables|/Game/ThirdPerson/Blueprints/BP_ThirdPersonCharacter.BP_ThirdPersonCharacter_C|SetRun%20speed _asbp_third_person_character (Variables|Default|GetInitial_Walk_Speed))
  (Variables|/Game/ThirdPerson/Blueprints/BP_ThirdPersonCharacter.BP_ThirdPersonCharacter_C|SetNotSteal%20Mana? _asbp_third_person_character true)
  (Variables|Default|SetStart/stop false)
  (Utilities|Time|ClearandInvalidateTimerbyHandle (Variables|Default|GetTimer)))

(event Custom|dying
  (if (<= (Variables|/Game/ThirdPerson/Blueprints/BP_Melia.BP_Melia_C|GetHP (Variables|Default|GetAs%20BP%20Melia)) 0.0)
    (Default|CoupDuDestin (Variables|Default|GetAs%20BP%20Melia))))

(event Custom|Steal%20Mana
  (bind _asbp_melia (Utilities|Casting|CastToBP_Melia (Game|GetPlayerCharacter 0)))
  (Variables|Default|SetAs%20BP%20Melia _asbp_melia)
  (Utilities|FlowControl|DoOnce false :!label _label
    (:Completed
      (if (Variables|Default|GetStart/stop)
        (Utilities|FlowControl|Delay (Variables|Default|GetDelay_Between_Ticks))
        (Variables|/Game/ThirdPerson/Blueprints/BP_Melia.BP_Melia_C|SetNotSteal%20Mana? (Variables|Default|GetAs%20BP%20Melia) false)
        (if (Variables|Default|GetStart/stop)
          (Variables|/Game/ThirdPerson/Blueprints/BP_Melia.BP_Melia_C|SetHP (Variables|Default|GetAs%20BP%20Melia) 0.0)
          (Default|Update (Variables|/Game/ThirdPerson/Blueprints/BP_Melia.BP_Melia_C|GetHUD (Variables|Default|GetAs%20BP%20Melia)) 0.0)
          (Default|ShowHud (Variables|Default|GetAs%20BP%20Melia))
          (CallFunction|Dying)
          (Utilities|FlowControl|Sequence
            (:then_0
              (goto _label Reset))
            (:then_1
              (CallFunction|StealMana)))
          (else
            (goto _label Reset)))
        (else
          (goto _label Reset))))))

(event Custom|Set%20speed
  (if (Variables|Default|GetStart/stop)
    (Default|ModifyWalkSpeed (Variables|Default|GetAs%20BP%20Melia) (Variables|Default|GetNew_Walk_Speed))))

(event EventBeginPlay)

(event Collision|EventActorBeginOverlap
  (params (OtherActor :type Actor%20Object%20Reference)))

(event EventTick
  (params (DeltaSeconds :type Float%20%28single-precision%29)))

(fn ConstructionScript)