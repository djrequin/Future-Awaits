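; BP_CheckPoint is a checkpoint actor that updates the player's respawn point when BP_Melia enters its box trigger.
; The first such overlap copies the checkpoint's root location and rotation, at unit scale, into Melia's RespawnPoint.
; It then calls SaveLevelRespawn on the Game_Instance_Future_Awaits reference cached at BeginPlay.
; A DoOnce with no reset limits each checkpoint to a single activation per actor instance.
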(event OnComponentBeginOverlap(Box)
  (params (OverlappedComponent :type Primitive%20Component%20Object%20Reference) (OtherActor :type Actor%20Object%20Reference) (OtherComp :type Primitive%20Component%20Object%20Reference) (OtherBodyIndex :type Integer) (bFromSweep :type Boolean) (SweepResult :type Hit%20Result%20Structure%20%28by%20ref%29))
  (bind _defaultsceneroot (Variables|Default|GetDefaultSceneRoot))
  (bind _returnvalue (Transformation|GetWorldTransform _defaultsceneroot))
  (bind _asbp_melia (Utilities|Casting|CastToBP_Melia OtherActor))
  (bind _output_get (Variables|Default|SetAs%20BP%20Melia _asbp_melia))
  (Utilities|FlowControl|DoOnce false
    (:Completed
      (Variables|/Game/ThirdPerson/Blueprints/BP_Melia.BP_Melia_C|SetRespawn_Point _output_get (Math|Transform|MakeTransform (.location _returnvalue) (.rotation _returnvalue) "1.000000,1.000000,1.000000"))
      (Default|SaveLevelRespawn (Variables|Default|GetAs%20Game%20Instance%20Future%20Awaits)))))

(event EventBeginPlay
  (bind _asgame_instance_future_awaits (Utilities|Casting|CastToGame_Instance_Future_Awaits (Game|GetGameInstance)))
  (Variables|Default|SetAs%20Game%20Instance%20Future%20Awaits _asgame_instance_future_awaits))

(fn ConstructionScript)