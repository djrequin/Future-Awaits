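; BP_Noeud is a prototype interactable that checks whether the player has collected every memory and announces the end of the game with debug prints.
; On BeginPlay it caches the player character as BP_Melia and enables a PrintInteracton flag.
; Its Interaction event compares Melia's MemoriesCollected to the length of the Memories array, printing a French game-over message on a match, otherwise both counts.
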(event EventBeginPlay
  (|CallParentFunction)
  (bind _asbp_melia (Utilities|Casting|CastToBP_Melia (Game|GetPlayerCharacter 0)))
  (Variables|Default|SetAs%20BP%20Melia_0 _asbp_melia)
  (Variables|Default|SetPrint_interacton true))

(event EventInteraction
  (bind _as_bp_melia_0 (Variables|Default|GetAs%20BP%20Melia_0))
  (bind _memories (Variables|Default|GetMemories))
  (bind _returnvalue (Utilities|Array|Length _memories))
  (bind _memories_collected (Variables|/Game/ThirdPerson/Blueprints/BP_Melia.BP_Melia_C|GetMemories_collected _as_bp_melia_0))
  (if (== _memories_collected _returnvalue)
    (Development|PrintString "le jeu est fini,gg")
    (else
      (Utilities|FlowControl|Sequence
        (:then_0
          (Development|PrintString (Utilities|String|Append "Souvenirs collectés : " (Utilities|String|ToString(Integer) _memories_collected))))
        (:then_1
          (Development|PrintString (Utilities|String|Append "Taille tableau : " (Utilities|String|ToString(Integer) _returnvalue))))))))

(fn ConstructionScript
  (|CallParentFunction))