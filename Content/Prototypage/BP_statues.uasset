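; Interactable statue that lets the player collect a memory ("souvenir") once, built on a parent that supplies its begin-play logic.
; It sets a collection prompt at start; the first interaction clears it, increments the character's Memories count, then shows and notifies the TFLucioles (fireflies) element.
; A one-in-five roll then plays a random quote through the dynamic UI, using parallel arrays for text, voice, speaker name and delay.
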(event EventBeginPlay
  (|CallParentFunction)
  (Variables|Default|SetText%20to%20print "-  Collecter les souvenirs."))

(event Collision|EventActorBeginOverlap
  (params (OtherActor :type Actor%20Object%20Reference)))

(event EventTick
  (params (DeltaSeconds :type Float%20%28single-precision%29)))

(event EventInteraction
  (bind _thirdpersoncharacter (Variables|Default|GetThirdPersonCharacter))
  (bind _tf_lucioles (Variables|/Game/ThirdPerson/Blueprints/BP_ThirdPersonCharacter.BP_ThirdPersonCharacter_C|GetTF/Lucioles _thirdpersoncharacter))
  (Utilities|FlowControl|DoOnce false
    (:Completed
      (Math|Integer|IncrementInt (Variables|/Game/ThirdPerson/Blueprints/BP_ThirdPersonCharacter.BP_ThirdPersonCharacter_C|GetMemories _thirdpersoncharacter)
        (:%20%20
          (Variables|Default|SetText%20to%20print "")
          (Widget|SetVisibility _tf_lucioles "Visible")
          (Default|GotMemories _tf_lucioles)
          (CallFunction|UseAQuote?))))))

(fn ConstructionScript
  (|CallParentFunction))

(fn UseAQuote?
  (if (== (Math|Random|RandomIntegerinRange 0 4) 0)
    (LocalVariables|SetArray_ref (Math|Random|RandomIntegerinRange 0 (- (Utilities|Array|Length (Variables|Default|GetQuote)) 1)))
    (Default|Initialize (Variables|/Game/ThirdPerson/Blueprints/BP_ThirdPersonCharacter.BP_ThirdPersonCharacter_C|GetDynamic_UI (Variables|Default|GetThirdPersonCharacter)) (Utilities|Array|MakeArray (Utilities|Array|Get(acopy) (Variables|Default|GetDelay) (LocalVariables|GetArray_ref))) (Utilities|Array|MakeArray (Utilities|Array|Get(acopy) (Variables|Default|GetVoice) (LocalVariables|GetArray_ref))) (Utilities|Array|MakeArray (Utilities|Array|Get(acopy) (Variables|Default|GetQuote) (LocalVariables|GetArray_ref))) (Utilities|Array|MakeArray (Utilities|Array|Get(acopy) (Variables|Default|GetName) (LocalVariables|GetArray_ref))))))