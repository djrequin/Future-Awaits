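; BP_Hp_Flowers is an interactable flower prop that, as wired, sets the player's HP to zero.
; BeginPlay caches the player character as BP_Melia, and DisplayName passes the prop's text to the supplied display widget.
; Interaction zeroes Melia's HP, updates her HUD and shows it.
; A clamped HpRegen heal and a DestroyActor call are left unconnected, so the flower neither heals nor destroys itself.
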(event EventBeginPlay
  (bind _asbp_melia (Utilities|Casting|CastToBP_Melia (Game|GetPlayerCharacter 0)))
  (Variables|Default|SetAs%20BP%20Melia _asbp_melia))

(event Collision|EventActorBeginOverlap
  (params (OtherActor :type Actor%20Object%20Reference)))

(event EventTick
  (params (DeltaSeconds :type Float%20%28single-precision%29)))

(event EventInteraction
  (bind _as_bp_melia (Variables|Default|GetAs%20BP%20Melia))
  (bind _output_get (Variables|/Game/ThirdPerson/Blueprints/BP_Melia.BP_Melia_C|SetHP _as_bp_melia 0.0))
  (Default|Update (Variables|/Game/ThirdPerson/Blueprints/BP_Melia.BP_Melia_C|GetHUD _as_bp_melia) _output_get)
  (Default|ShowHud _as_bp_melia))

(event EventDisplayName
  (params (Widget%20%28Tirer%20"show"%29 :type WB%20Interaction%20Button%20Object%20Reference))
  (Default|Show Widget%20%28Tirer%20"show"%29 (Variables|Default|GetText)))

(fn ConstructionScript)