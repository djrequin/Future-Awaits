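; BP_Corrupted_Obstacle is an obstacle tied to a set of corrupted flowers that removes itself once enough deaths are reported.
; On BeginPlay it assigns itself as the Obstacle reference on each entry in its Flowers array.
; Each call to its Death event increments the Line counter, and the actor is destroyed when that count reaches the number of flowers.
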(event Custom|Death
  (Math|Integer|IncrementInt (Variables|Default|GetLine)
    (:%20%20
      (if (>= (Variables|Default|GetLine) (Utilities|Array|Length (Variables|Default|GetFlowers)))
        (Actor|DestroyActor)))))

(event EventBeginPlay
  (for _array_element (Variables|Default|GetFlowers)
    (Variables|/Game/Prototypage/Explo/Corrupted_flowers/BP_Corrupted_Flower.BP_Corrupted_Flower_C|SetObstacle _array_element self)))

(event Collision|EventActorBeginOverlap
  (params (OtherActor :type Actor%20Object%20Reference)))

(event EventTick
  (params (DeltaSeconds :type Float%20%28single-precision%29)))

(fn ConstructionScript)