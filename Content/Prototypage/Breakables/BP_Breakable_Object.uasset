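; Breakable prop that, when shot, spawns a dark-magic blink effect at its location and scale, then destroys itself.
; On BeginPlay, a breakable type selects the obstacle look (rock or root walls, dead tree, cracked rock, Léni wall), setting mesh and material.
; The mesh's non-default world scale and rotation are captured and reapplied, unless override flags keep the preset values.
; The construction script only calls its parent, and the Interaction event is empty.
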(event EventBeginPlay
  (Variables|Default|SetPrint_interacton false)
  (SettingBreakable|TestMesh))

(event EventInteraction)

(event EventShotEvent
  (params (Impact_Location :type Vector :default "0, 0, 0"))
  (Niagara|SpawnSystematLocation "/Game/BlinkAndDashVFX/VFX_Niagara/NS_Blink_DarkMagic1.NS_Blink_DarkMagic1" (Transformation|GetActorLocation) "0, 0, 0" (Transformation|GetWorldScale (Variables|Default|GetCube_0)))
  (Actor|DestroyActor))

(fn ConstructionScript
  (|CallParentFunction))

(fn Init
  (params (Type :type Enum_Breakables%20Enum :default "NewEnumerator0"))
  (switch Utilities|FlowControl|Switch|SwitchonEnum_Breakables Type
    (:NewEnumerator0
      (CallFunction|SetAll "/Game/Assets/WallRock/SM_WallRock.SM_WallRock" "/Game/Assets/WallRock/M_WallRock.M_WallRock"))
    (:NewEnumerator1
      (CallFunction|SetAll "/Game/Assets/Root/Root_Wall/SM_WallRoot.SM_WallRoot" "/Game/Assets/Root/Root_Wall/M_WallRoot.M_WallRoot"))
    (:NewEnumerator2
      (CallFunction|SetAll "/Game/Assets/DeathTree/SM_DeathTree.SM_DeathTree" "/Game/Assets/DeathTree/M_DeathTree.M_DeathTree"))
    (:NewEnumerator3
      (CallFunction|SetAll "/Game/Assets/BrokenRock/SM_BrokenRock.SM_BrokenRock" "/Game/Assets/BrokenRock/M_BrokenRock.M_BrokenRock"))
    (:NewEnumerator4
      (CallFunction|SetAll "/Game/LD/Proto/MurDeLeni.MurDeLeni"))))

(fn SetAll
  (params (Mesh :type Static%20Mesh%20Object%20Reference) (Mat :type Material%20Object%20Reference))
  (bind _cube_0 (Variables|Default|GetCube_0))
  (Components|StaticMesh|SetStaticMesh _cube_0 Mesh)
  (Rendering|Material|SetMaterial _cube_0 0 Mat)
  (Transformation|SetWorldScale3D _cube_0 (Variables|SettingBreakable|GetWanted_Scale))
  (Transformation|SetWorldRotation _cube_0 (Variables|SettingBreakable|GetWanted_Rota) false false))

(fn CheckScale
  (bind _cube_0 (Variables|Default|GetCube_0))
  (bind _returnvalue (Transformation|GetWorldScale _cube_0))
  (if (Variables|SettingBreakable|GetOverride_World_Scale)
    _
    (elif (Utilities|Operators|EqualEqual _returnvalue "1.000000,1.000000,1.000000" 0.0)
      _
      (else
        (Variables|SettingBreakable|SetWanted_Scale _returnvalue))))
  (return))

(fn CheckRota
  (bind _cube_0 (Variables|Default|GetCube_0))
  (bind _returnvalue (Transformation|GetWorldRotation _cube_0))
  (if (Variables|SettingBreakable|GetOverride_World_Rotation)
    _
    (elif (Utilities|Operators|EqualEqual :A _returnvalue)
      _
      (else
        (Variables|SettingBreakable|SetWanted_Rota _returnvalue))))
  (return))

(fn TestMesh
  (CallFunction|CheckScale)
  (CallFunction|CheckRota)
  (CallFunction|Init (Variables|SettingBreakable|GetBrekable_Type)))