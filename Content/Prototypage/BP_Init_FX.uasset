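; BP_Init_FX is a short-lived actor that spawns a batch of Niagara effects on BeginPlay, apparently to initialise them at game start.
; A Sequence fires the blink, flower, rewind and Lucioles systems together with no spawn location set.
; The flower and rewind systems are deactivated after a short delay, with both Melia rewind variants sharing one delay.
; The actor destroys itself shortly afterwards.
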(event EventBeginPlay
  (Utilities|FlowControl|Sequence
    (:then_0
      (bind _returnvalue (Niagara|SpawnSystematLocation "/Game/Prototypage/Corrupted_flowers/VFX/NS_LargeFlower_Open.NS_LargeFlower_Open" "0, 0, 0"))
      (Utilities|FlowControl|Delay 2.0)
      (Components|Activation|Deactivate _returnvalue))
    (:then_1
      (Niagara|SpawnSystematLocation "/Game/BlinkAndDashVFX/VFX_Niagara/NS_Blink_DarkMagic1.NS_Blink_DarkMagic1" "0, 0, 0"))
    (:then_2
      (Niagara|SpawnSystematLocation "/Game/BlinkAndDashVFX/VFX_Niagara/NS_Blink_DarkMagic.NS_Blink_DarkMagic" "0, 0, 0"))
    (:then_3
      (Niagara|SpawnSystematLocation "/Game/BlinkAndDashVFX/VFX_Niagara/NS_Blink_Psionic2.NS_Blink_Psionic2" "0, 0, 0"))
    (:then_4
      (Niagara|SpawnSystematLocation "/Game/BlinkAndDashVFX/VFX_Niagara/NS_Blink_Psionic.NS_Blink_Psionic" "0, 0, 0"))
    (:then_5
      (Niagara|SpawnSystematLocation "/Game/BlinkAndDashVFX/VFX_Niagara/TF_blink.TF_blink" "0, 0, 0"))
    (:then_6
      (bind _returnvalue_2 (Niagara|SpawnSystematLocation "/Game/ThirdPerson/Blueprints/SkillRewind/VFX/NS_RewindIdle.NS_RewindIdle" "0, 0, 0"))
      (Utilities|FlowControl|Delay 2.0)
      (Components|Activation|Deactivate _returnvalue_2))
    (:then_7
      (bind _returnvalue_3 (Niagara|SpawnSystematLocation "/Game/ThirdPerson/Blueprints/SkillRewind/VFX/NS_RewindMelia.NS_RewindMelia" "0, 0, 0"))
      (Utilities|FlowControl|Delay 2.0 :!label _label)
      (Components|Activation|Deactivate _returnvalue_3))
    (:then_8
      (Niagara|SpawnSystematLocation "/Game/BlinkAndDashVFX/VFX_Niagara/Lucioles.Lucioles" "0, 0, 0"))
    (:then_9
      (bind _returnvalue_4 (Niagara|SpawnSystematLocation "/Game/ThirdPerson/Blueprints/SkillRewind/VFX/NS_RewindMelia1.NS_RewindMelia1" "0, 0, 0"))
      (goto _label))
    (:then_11
      (Utilities|FlowControl|Delay 3.0)
      (Actor|DestroyActor))))

(fn ConstructionScript)