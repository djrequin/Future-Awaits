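; Prototype slow-effect item: a physics cube that is unfrozen while slowed and freezes again afterwards.
; StartSlow cancels any pending timer and enables physics simulation on the cube.
; EndSlow starts a timer that, followed by a fixed delay, switches physics off again.
; ShotEvent applies a clamped velocity-change impulse built from the cube's world location plus the scaled input vector.
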(event Custom|end%20unfroze
  (Utilities|FlowControl|Delay 5.0)
  (Physics|SetSimulatePhysics (Variables|Default|GetCube) false)
  (Variables|Default|SetIs%20unfroze%20? false)
  (Development|PrintString "frozen" true true "(R=1.000000,G=0.048928,B=0.000000,A=1.000000)"))

(event EventShotEvent
  (params (Forward%20vector :type Float%20%28double-precision%29) (fv :type Vector :default "0, 0, 0"))
  (if true
    (Physics|AddImpulse (Variables|Default|GetCube) (Math|Vector|ClampVectorSize (+ (Transformation|GetWorldLocation (Variables|Default|GetCube)) (* fv 1e+02)) 0.0 1e+03) "None" true)))

(event EventEndSlow
  (bind _returnvalue (Utilities|Time|SetTimerbyEvent (delegate Custom|end%20unfroze) (Variables|Default|GetTime)))
  (Variables|Default|Settimer _returnvalue))

(event EventStartSlow
  (Utilities|Time|ClearandInvalidateTimerbyHandle (Variables|Default|Gettimer))
  (Physics|SetSimulatePhysics (Variables|Default|GetCube) true)
  (Variables|Default|SetIs%20unfroze%20? true)
  (Development|PrintString "Unfrozen"))

(fn ConstructionScript)