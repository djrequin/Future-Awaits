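; BP_Empty_needle is an empty needle variant that marks itself Empty on BeginPlay and starts a floating bob animation.
; A FlipFlop alternately plays a half-rate Timeline forward and in reverse, lerping the Cone's relative Z to move it slightly up and down.
; The Timeline's Finished output calls Floating again to repeat the motion until StopMove is set.
; The parent BeginPlay call is left unconnected.
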(event Custom|floating
  (if (not (Variables|Default|GetStopMove))
    (Components|Timeline|SetPlayRate (Variables|Default|GetTimeline) 0.5)
    (Utilities|FlowControl|FlipFlop
      (:A
        (bind _newtrack_0 (Timeline|Timeline PlayFromStart)
          (:Update
            (Transformation|SetRelativeLocation (Variables|Default|GetCone) (Math|Vector|MakeVector 0.0 0.0 (Math|Float|Lerp 0.0 3.0 _newtrack_0)) false false))
          (:Finished
            (CallFunction|Floating))))
      (:B
        (Timeline|Timeline ReverseFromEnd)))))

(event EventBeginPlay
  (Variables|Default|Setempty? true)
  (CallFunction|Floating))

(event Collision|EventActorBeginOverlap
  (params (OtherActor :type Actor%20Object%20Reference)))

(event EventTick
  (params (DeltaSeconds :type Float%20%28single-precision%29)))

(fn ConstructionScript
  (|CallParentFunction))