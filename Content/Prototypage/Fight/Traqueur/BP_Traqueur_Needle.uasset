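; Needle actor of the Traqueur fight that hurts the player on contact and can be destroyed through a shot event.
; Box overlap with BP_ThirdPersonCharacter fires once, dealing damage and stealing mana before the needle destroys itself.
; ShotEvent spawns an enlarged explosion at the Cone's transform, plays damage force feedback on the first player controller, then destroys the needle.
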(event OnComponentBeginOverlap(Box)
  (params (OverlappedComponent :type Primitive%20Component%20Object%20Reference) (OtherActor :type Actor%20Object%20Reference) (OtherComp :type Primitive%20Component%20Object%20Reference) (OtherBodyIndex :type Integer) (bFromSweep :type Boolean) (SweepResult :type Hit%20Result%20Structure%20%28by%20ref%29))
  (bind _asbp_third_person_character (Utilities|Casting|CastToBP_ThirdPersonCharacter OtherActor))
  (Utilities|FlowControl|DoOnce false
    (:Completed
      (Default|TakeDamages _asbp_third_person_character 2.0 0 true 5.0)
      (Actor|DestroyActor))))

(event EventBeginPlay)

(event Collision|EventActorBeginOverlap
  (params (OtherActor :type Actor%20Object%20Reference)))

(event EventTick
  (params (DeltaSeconds :type Float%20%28single-precision%29)))

(event EventShotEvent
  (bind _cone (Variables|Default|GetCone))
  (bind _returnvalue (Transformation|GetWorldTransform _cone))
  (Effects|SpawnEmitteratLocation "/Game/StarterContent/Particles/P_Explosion.P_Explosion" (.location _returnvalue) (.rotation _returnvalue) (* (.scale _returnvalue) 5e+01))
  (Game|Feedback|ClientPlayForceFeedback (Game|GetPlayerController 0) "/Game/ThirdPerson/Blueprints/FF/FF_Damages.FF_Damages" "None" false false false)
  (Actor|DestroyActor))

(fn ConstructionScript)