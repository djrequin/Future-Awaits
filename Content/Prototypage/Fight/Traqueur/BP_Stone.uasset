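; BP_Stone is a stone hazard in the Traqueur fight prototype that deals damage and steals mana on overlap.
; A Timeline started on BeginPlay raises the Cone by a fixed step each update, independent of any curve value.
; The first Box overlap with a BPI_Ennemy_damages actor sends damage; if that actor is BP_Melia, it clears Father's CanKeep and destroys itself.
; ShotEvent is empty, and the explosion and force feedback logic is unconnected.
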(event OnComponentBeginOverlap(Box)
  (params (OverlappedComponent :type Primitive%20Component%20Object%20Reference) (OtherActor :type Actor%20Object%20Reference) (OtherComp :type Primitive%20Component%20Object%20Reference) (OtherBodyIndex :type Integer) (bFromSweep :type Boolean) (SweepResult :type Hit%20Result%20Structure%20%28by%20ref%29))
  (if (Utilities|DoesObjectImplementInterface OtherActor "/Game/Prototypage/Fight/BPI_Ennemy_damages.BPI_Ennemy_damages_C")
    (Utilities|FlowControl|DoOnce false
      (:Completed
        (Class|BPIEnnemyDamages|DealDamages(Message) OtherActor (Variables|Default|GetDamages%20Dealt) true (Variables|Default|GetMana%20Taken))
        (Utilities|Casting|CastToBP_Melia OtherActor)
        (Variables|/Game/Prototypage/Fight/Traqueur/BP_Traqueur.BP_Traqueur_C|SetCan%20keep%20? (Variables|Default|GetFather) false)
        (Actor|DestroyActor)))))

(event EventBeginPlay
  (bind _cone (Variables|Default|GetCone))
  (bind _returnvalue (Transformation|GetWorldTransform _cone))
  (Timeline|Timeline PlayFromStart
    (:Update
      (Transformation|SetWorldTransform _cone (Math|Transform|MakeTransform (Math|Vector|MakeVector (.x (.location _returnvalue)) (.y (.location _returnvalue)) (+ (.z (.location _returnvalue)) 7.0)) (.rotation _returnvalue) (.scale _returnvalue)) false false))))

(event EventShotEvent)

(fn ConstructionScript)