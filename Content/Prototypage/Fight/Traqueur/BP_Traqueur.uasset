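; Traqueur enemy character that hands patrol points and PawnSensing detection to AIC_Traqueur, switching to chase speed until a loss timer expires.
; It attacks with a charged needle projectile, a mana-stealing short-range overlap hit and a repeating stone spawn beneath the player.
; Hits can trigger a smoke state making it invisible, invincible and unlockable.
; Long attacks open timed vulnerability windows, and a freeze order removes the smoke.
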(event OnSeePawn(PawnSensing_0)
  (params (Pawn :type Pawn%20Object%20Reference))
  ;[1 1 1] vision
  (bind _asbp_third_person_character (Utilities|Casting|CastToBP_ThirdPersonCharacter Pawn))
  (Default|Enter/exitFight _asbp_third_person_character true)
  (Utilities|Time|ClearandInvalidateTimerbyHandle (Variables|Detection|GetTimer))
  (Default|PlayerDetected (Variables|Default|GetAIC) true)
  (bind _returnvalue (Utilities|Time|SetTimerbyEvent (delegate Custom|lose_player) (Variables|Detection|GetPlayer_loss%20time)))
  (Variables|Detection|SetTimer _returnvalue)
  (CallFunction|ChangeWalkSpeed "NewEnumerator1"))

(event OnComponentBeginOverlap(attack_short)
  (params (OverlappedComponent :type Primitive%20Component%20Object%20Reference) (OtherActor :type Actor%20Object%20Reference) (OtherComp :type Primitive%20Component%20Object%20Reference) (OtherBodyIndex :type Integer) (bFromSweep :type Boolean) (SweepResult :type Hit%20Result%20Structure%20%28by%20ref%29))
  ;[1 1 1] Shprt attack
  (if (and (Variables|Short_attack|GetShort_range_active?) (Utilities|DoesObjectImplementInterface OtherActor "/Game/Prototypage/Fight/BPI_Ennemy_damages.BPI_Ennemy_damages_C"))
    (Utilities|FlowControl|DoOnce false :!label _label
      (:Completed
        (Class|BPIEnnemyDamages|DealDamages(Message) OtherActor (Variables|Short_attack|GetDamages%20Dealt%28short%29) true (Variables|Short_attack|GetMana%20Taken%28short%29))
        (Utilities|FlowControl|Delay 2.0)
        (goto _label Reset)))))

(event Custom|lose_player
  ;[1 1 1] vision
  (Default|PlayerDetected (Variables|Default|GetAIC) false)
  (Default|Enter/exitFight (Variables|Default|GetAs%20BP%20Third%20Person%20Character) false)
  (Development|PrintString "Lost"))

(event Custom|Long_attack
  (bind _needle_ref (Variables|Default|GetNeedle_ref))
  (bind _returnvalue (Transformation|GetWorldTransform _needle_ref))
  ;[1 1 1] Long attack
  (bind _returnvalue_2 (Game|SpawnActorfromClass "/Game/Prototypage/Fight/Traqueur/BP_empty.BP_empty_C" (Math|Transform|MakeTransform (.location _returnvalue) (.rotation _returnvalue) "1.000000,1.000000,1.000000") "Undefined" "MultiplyWithRoot" 0 0))
  (Transformation|AttachComponentToComponent _returnvalue_2 (Variables|Default|GetNeedle_ref) "None" "SnapToTarget" "SnapToTarget" "KeepWorld" true)
  (bind _output_get (Variables|1stLongAttack(needle)|SetNeedle _returnvalue_2))
  (Variables|1stLongAttack(needle)|Setscale (.scale (Transformation|GetActorTransform _output_get)))
  (bind _newtrack_0 (Timeline|charge PlayFromStart)
    (:Update
      (Utilities|IsValid (Variables|1stLongAttack(needle)|GetNeedle)
        (:Is%20Valid
          (Transformation|SetActorTransform (Variables|1stLongAttack(needle)|GetNeedle) (Math|Transform|MakeTransform (.location (Transformation|GetActorTransform (Variables|1stLongAttack(needle)|GetNeedle))) (.rotation (Transformation|GetActorTransform (Variables|1stLongAttack(needle)|GetNeedle))) (* (Variables|1stLongAttack(needle)|Getscale) (Math|Float|Lerp 0.4 3.0 _newtrack_0))))
          (Utilities|FlowControl|Delay (Math|Random|RandomFloatinRange 1.0 4.0))
          (CallFunction|Shoot)
          (Utilities|StartVulnerability (Variables|1stLongAttack(needle)|GetVulnerability%20Time%201st_long) false))))))

(event Custom|shoot
  (bind _needle (Variables|1stLongAttack(needle)|GetNeedle))
  (bind _returnvalue (Transformation|GetActorTransform _needle))
  ;[1 1 1] Long attack
  (bind _returnvalue_2 (Game|SpawnActorfromClass "/Game/Prototypage/Fight/Traqueur/BP_Traqueur_Needle.BP_Traqueur_Needle_C" (Math|Transform|MakeTransform (.location _returnvalue) (Math|Rotator|FindLookatRotation (Transformation|GetActorLocation _needle) (Transformation|GetActorLocation (Variables|/Game/Prototypage/Fight/Traqueur/AIC_Traqueur.AIC_Traqueur_C|GetAs%20BP%20Melia (Variables|Default|GetAIC)))) (.scale _returnvalue)) "Undefined" "MultiplyWithRoot" 0 0))
  (Utilities|IsValid _returnvalue_2
    (:Is%20Valid
      (Components|Activation|Activate (Variables|/Game/Prototypage/Fight/Traqueur/BP_Traqueur_Needle.BP_Traqueur_Needle_C|GetProjectileMovement _returnvalue_2) false)
      (Actor|DestroyActor _needle))))

(event Custom|Long_attack2
  (bind _as_bp_melia (Variables|Default|GetAs%20BP%20Melia))
  (bind _capsulecomponent (Variables|/Script/Engine.Character|GetCapsuleComponent _as_bp_melia))
  (bind _returnvalue (Transformation|GetWorldTransform _capsulecomponent))
  ;[1 1 1] 2nd long attack
  (Utilities|FlowControl|Delay (Variables|2ndLong(Stones)|Gettime_before_spawn))
  (CallFunction|Spawn)
  (Development|PrintString "stones")
  (bind _result (Math|Integer|IncrementInt (Variables|2ndLong(Stones)|GetCurrent_times))
    (:%20%20
      (if (>= _result (Variables|2ndLong(Stones)|Getmax%20times))
        (CallFunction|ResetLong2)
        (else
          (CallFunction|LongAttack2)
          (Utilities|FlowControl|DoOnce false) ; enters at Reset
        )))))

(event Custom|spawn
  (bind _as_bp_melia (Variables|Default|GetAs%20BP%20Melia))
  (bind _capsulecomponent (Variables|/Script/Engine.Character|GetCapsuleComponent _as_bp_melia))
  (bind _returnvalue (Transformation|GetWorldTransform _capsulecomponent))
  ;[1 1 1] 2nd long attack
  (Utilities|FlowControl|DoOnce false
    (:Completed
      (if (Variables|2ndLong(Stones)|GetCan%20keep%20?)
        (bind _returnvalue_2 (Game|SpawnActorfromClass "/Game/Prototypage/Fight/Traqueur/BP_Stone.BP_Stone_C" (Math|Transform|MakeTransform (Math|Vector|MakeVector (.x (.location _returnvalue)) (.y (.location _returnvalue)) (- (.z (.location _returnvalue)) 3.3e+02)) (.rotation _returnvalue) (.scale _returnvalue)) "Undefined" "MultiplyWithRoot" 0 0))
        (Variables|/Game/Prototypage/Fight/Traqueur/BP_Stone.BP_Stone_C|SetFather _returnvalue_2 self)))))

(event Custom|reset%20long2
  ;[1 1 1] 2nd long attack
  (Variables|2ndLong(Stones)|SetCurrent_times 0)
  (Variables|2ndLong(Stones)|SetCan%20keep%20? true))

(event Custom|Use%202nd%20long
  ;[1 1 1] 2nd long attack
  (Utilities|StartVulnerability (Variables|2ndLong(Stones)|GetVulnerability%20Time%202nd%20long) true
    (:NewParam3
      (CallFunction|LongAttack2))))

(event EventBeginPlay
  (|CallParentFunction)
  (CallFunction|GetPatrolLocations)
  (bind _asaic_traqueur (Utilities|Casting|CastToAIC_Traqueur (AI|GetAIController self)))
  (Variables|Default|SetAIC _asaic_traqueur)
  (Variables|/Game/Prototypage/Fight/Traqueur/AIC_Traqueur.AIC_Traqueur_C|SetTraqueur _asaic_traqueur self))

(event EventHitEvent
  ;[1 1 1] Should start smoke ?
  (Default|PlayerDetected (Variables|Default|GetAIC) true)
  (if (>= (Variables|Default|GetCurrent_Hit) (* (Variables|Default|GetHit_Numbers) 0.5))
    (Utilities|StartSmoke :!label _label)
    (elif (<= (Math|Random|RandomIntegerinRange 1 100) 10)
      (goto _label))))

(event EventFreezeOrdrer
  (Default|Freeze (Variables|Default|GetAIC))
  (Utilities|StopSmoke))

(fn ConstructionScript
  (|CallParentFunction))

(fn GetPatrolLocations
  (for _array_element (Variables|Patrol|GetPatrol-points)
    (Utilities|IsValid _array_element
      (:Is%20Valid
        (Utilities|Array|Add (Variables|Patrol|GetPatrol_positions) (Transformation|GetWorldLocation (Variables|/Game/Prototypage/Fight/Patrol_points.Patrol_points_C|GetDefaultSceneRoot _array_element)))))))

(fn ChangeWalkSpeed
  (params (enum :type Enum_speeds%20Enum :default "NewEnumerator0"))
  (switch Utilities|FlowControl|Switch|SwitchonEnum_speeds enum
    (:NewEnumerator0
      (LocalVariables|SetSpeed (Variables|speed|GetPatrol_speed)))
    (:NewEnumerator1
      (LocalVariables|SetSpeed (Variables|speed|GetChase_speed))))
  (Variables|/Script/Engine.CharacterMovementComponent|SetMaxWalkSpeed (Variables|Character|GetCharacterMovement) (LocalVariables|GetSpeed)))