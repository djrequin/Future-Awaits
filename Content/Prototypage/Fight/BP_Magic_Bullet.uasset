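; BP_Magic_Bullet is a projectile that produces impact effects and notifies shootable actors it touches, unless its Empty flag is set.
; Each tick, a short forward box trace ignoring the player and current zone manager triggers explosion particles and camera shake, plus a one-time impact sound.
; Separately, collision overlap with a BPI_Projectile_Interface actor sends ShotEventMessage once, shakes the camera and destroys the bullet.
; A trace hit alone leaves the bullet alive.
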(event OnComponentBeginOverlap(Collision)
  (params (OverlappedComponent :type Primitive%20Component%20Object%20Reference) (OtherActor :type Actor%20Object%20Reference) (OtherComp :type Primitive%20Component%20Object%20Reference) (OtherBodyIndex :type Integer) (bFromSweep :type Boolean) (SweepResult :type Hit%20Result%20Structure%20%28by%20ref%29))
  (Variables|Default|SetActor%20location (Transformation|GetActorLocation OtherActor))
  (if (not (Variables|Default|Getempty?))
    (if (Utilities|DoesObjectImplementInterface OtherActor "/Game/ThirdPerson/Blueprints/Interfaces/BPI_Projectile_Interface.BPI_Projectile_Interface_C")
      (Utilities|FlowControl|DoOnce false
        (:Completed
          (Class|BPIProjectileInterface|ShotEvent(Message) OtherActor)
          (Default|CameraShake (Variables|Default|GetAs%20BP%20Third%20Person%20Character) (Transformation|GetWorldLocation (Variables|Default|GetDefaultSceneRoot)) true)
          (Actor|DestroyActor))))))

(event EventBeginPlay
  (bind _asbp_third_person_character (Utilities|Casting|CastToBP_ThirdPersonCharacter (Game|GetPlayerCharacter 0)))
  (Variables|Default|SetAs%20BP%20Third%20Person%20Character _asbp_third_person_character))

(event EventTick
  (params (DeltaSeconds :type Float%20%28single-precision%29))
  (bind _returnvalue (Transformation|GetActorLocation))
  (bind _defaultsceneroot (Variables|Default|GetDefaultSceneRoot))
  (bind _returnvalue_2 (Transformation|GetWorldLocation _defaultsceneroot))
  (if (not (Variables|Default|Getempty?))
    (bind (_outhit _returnvalue_3) (Class|KismetSystemLibrary|BoxTraceSingleforObjects _returnvalue (+ _returnvalue (* (Transformation|GetActorForwardVector) 8e+01)) "5.000000,0.000000,10.000000" "0, 0, 0" (Utilities|Array|MakeArray "ObjectTypeQuery1" "ObjectTypeQuery7" "ObjectTypeQuery2" "ObjectTypeQuery11" "ObjectTypeQuery1" "ObjectTypeQuery10") false (Utilities|Array|MakeArray self (Variables|Default|GetAs%20BP%20Third%20Person%20Character) (Variables|/Game/ThirdPerson/Blueprints/BP_ThirdPersonCharacter.BP_ThirdPersonCharacter_C|GetCurrentZoneManager (Variables|Default|GetAs%20BP%20Third%20Person%20Character)) 0) "None" true))
    (if _returnvalue_3
      (Effects|SpawnEmitteratLocation "/Game/StarterContent/Particles/P_Explosion.P_Explosion" (.Location (Collision|BreakHitResult _outhit)))
      (Default|CameraShake (Variables|Default|GetAs%20BP%20Third%20Person%20Character) _returnvalue_2 true)
      (Utilities|FlowControl|DoOnce false
        (:Completed
          (Audio|SpawnSoundatLocation (Variables|Default|GetNeedle_impact) _returnvalue_2 "0, 0, 0" 1.0 1.0 0.0 (Variables|Default|GetAttenuation%20Settings) 0))))))

(fn ConstructionScript
  (|CallParentFunction))