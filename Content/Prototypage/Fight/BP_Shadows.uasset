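; Shadow enemy that patrols, chases the player and attacks to deal damage and steal mana.
; AIMoveTo drives random-point patrols; PawnSensing triggers a chase, with a looping timer that sends it back to its spawn position after a few seconds.
; A box overlap runs a delayed attack loop while the player stays inside, then resumes the chase.
; Kill increments the linked CorruptedTF's kill count and triggers its all-enemies-dead check.
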(event OnSeePawn(PawnSensing_0)
  (params (Pawn :type Pawn%20Object%20Reference))
  (Utilities|Casting|CastToBP_ThirdPersonCharacter Pawn)
  (CallFunction|Chase)
  (Utilities|FlowControl|DoOnce false
    (:Completed
      (CallFunction|Verif))))

(event OnComponentBeginOverlap(Box)
  (params (OverlappedComponent :type Primitive%20Component%20Object%20Reference) (OtherActor :type Actor%20Object%20Reference) (OtherComp :type Primitive%20Component%20Object%20Reference) (OtherBodyIndex :type Integer) (bFromSweep :type Boolean) (SweepResult :type Hit%20Result%20Structure%20%28by%20ref%29))
  (bind _asbp_third_person_character (Utilities|Casting|CastToBP_ThirdPersonCharacter OtherActor))
  (Variables|Default|SetAs%20BP%20Third%20Person%20Character_0 _asbp_third_person_character)
  (Utilities|FlowControl|DoOnce false
    (:Completed
      (Variables|Default|SetPlayer%20is%20in%20box%20? true)
      (CallFunction|Attack))))

(event OnComponentEndOverlap(Box)
  (params (OverlappedComponent :type Primitive%20Component%20Object%20Reference) (OtherActor :type Actor%20Object%20Reference) (OtherComp :type Primitive%20Component%20Object%20Reference) (OtherBodyIndex :type Integer))
  (Utilities|Casting|CastToBP_ThirdPersonCharacter OtherActor)
  (Variables|Default|SetPlayer%20is%20in%20box%20? false)
  (Utilities|FlowControl|DoOnce false) ; enters at Reset
)

(event Custom|Patrol
  (if (not (Variables|Default|Getstopped?))
    (Variables|/Script/Engine.CharacterMovementComponent|SetMaxWalkSpeed (Variables|Character|GetCharacterMovement) (Variables|Default|GetPatrol_Speed))
    (AI|AIMoveTo self (.RandomLocation (AI|Navigation|GetRandomReachablePointinRadius (Transformation|GetActorLocation) (Variables|Default|GetPatrol%20radius) 0 0)) 0 5.0 false
      (:OnSuccess
        (CallFunction|Patrol)))))

(event Custom|Chase_Player
  (if (not (Variables|Default|Getstopped?))
    (Variables|/Script/Engine.CharacterMovementComponent|SetMaxWalkSpeed (Variables|Character|GetCharacterMovement) (Variables|Default|GetChase_speed))
    (AI|AIMoveTo self "0, 0, 0" (Game|GetPlayerCharacter 0) 5.0 false)))

(event Custom|Verif
  (bind _returnvalue (Utilities|Time|SetTimerbyEvent (delegate Custom|ChaseTime) 1.0 true))
  (Variables|Default|SetTimer _returnvalue))

(event Custom|ChaseTime
  (if (not (Variables|Default|Getstopped?))
    (if (< (Variables|Default|GetChase_Delay) 4.0)
      (bind _result (Math|Float|IncrementFloat (Variables|Default|GetChase_Delay))
        (:%20%20
          (Variables|Default|SetChase_Delay _result)))
      (else
        (Utilities|Time|ClearandInvalidateTimerbyHandle (Variables|Default|GetTimer))
        (Components|Movement|StopMovementImmediately (Variables|Character|GetCharacterMovement))
        (CallFunction|BacktoStart)
        (Variables|Default|SetChase_Delay 0.0)
        (CallFunction|Reset)))))

(event Custom|reset
  (Utilities|FlowControl|DoOnce false) ; enters at Reset
)

(event Custom|Attack
  (if (not (Variables|Default|Getstopped?)) :!label _label
    (if (Variables|Default|GetPlayer%20is%20in%20box%20?)
      (Utilities|FlowControl|Delay (Variables|Default|GetTime%20before%20attacking))
      (if (Variables|Default|GetPlayer%20is%20in%20box%20?)
        (Default|TakeDamages (Variables|Default|GetAs%20BP%20Third%20Person%20Character_0) (Variables|Default|Getattack_damages) self true (Variables|Default|GetMana_taken))
        (goto _label)
        (else
          (CallFunction|Chase)))
      (else
        (CallFunction|Chase)))))

(event Custom|back%20to%20start
  (AI|AIMoveTo self (Variables|Default|GetStart%20position) 0 5.0 false :!label _label
    (:OnSuccess
      (CallFunction|Patrol))
    (:OnFail
      (Utilities|FlowControl|Delay (Utilities|Time|GetWorldDeltaSeconds))
      (if true
        (goto _label)))))

(event EventBeginPlay
  (|CallParentFunction)
  (CallFunction|Patrol)
  (Variables|Default|SetStart%20position (Transformation|GetWorldLocation (Variables|Default|GetCapsuleComponent))))

(event EventKill
  (bind _corrupted_tf (Variables|Default|GetCorrupted_TF))
  (if (Variables|Default|GetCorrupted_TF?)
    (bind _result (Math|Integer|IncrementInt (Variables|/Game/Prototypage/Frozen_zone/BP_Corrupted_Tf.BP_Corrupted_Tf_C|GetEnnemies_Killed _corrupted_tf))
      (:%20%20
        (Variables|/Game/Prototypage/Frozen_zone/BP_Corrupted_Tf.BP_Corrupted_Tf_C|SetEnnemies_Killed _corrupted_tf _result)
        (Default|AllEnnemiesDead? _corrupted_tf)))))

(event EventChase
  (CallFunction|ChasePlayer))

(fn ConstructionScript
  (|CallParentFunction))