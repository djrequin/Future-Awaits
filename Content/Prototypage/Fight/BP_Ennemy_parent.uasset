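; Parent enemy Blueprint that takes a set number of hits, then freezes and becomes open to a player finisher.
; Shots call Marker, which counts hits unless invincible, updates the marks widget and, at the limit, stops movement and applies a gold material.
; A trigger box registers the killable enemy on the player, letting Finisher kill it, release lock-on and destroy it.
; Empty hit and freeze events serve as hooks for child enemies.
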(event OnComponentBeginOverlap(Box)
  (params (OverlappedComponent :type Primitive%20Component%20Object%20Reference) (OtherActor :type Actor%20Object%20Reference) (OtherComp :type Primitive%20Component%20Object%20Reference) (OtherBodyIndex :type Integer) (bFromSweep :type Boolean) (SweepResult :type Hit%20Result%20Structure%20%28by%20ref%29))
  ;[1 0.4757 0.9041] is in player's box
  (bind _asbp_third_person_character (Utilities|Casting|CastToBP_ThirdPersonCharacter OtherActor))
  (if (Variables|Common_conditions|GetCan%20be%20Killed?)
    (Variables|/Game/ThirdPerson/Blueprints/BP_ThirdPersonCharacter.BP_ThirdPersonCharacter_C|SetEnnemy_In_Box _asbp_third_person_character self)))

(event OnComponentEndOverlap(Box)
  (params (OverlappedComponent :type Primitive%20Component%20Object%20Reference) (OtherActor :type Actor%20Object%20Reference) (OtherComp :type Primitive%20Component%20Object%20Reference) (OtherBodyIndex :type Integer))
  ;[1 0.4757 0.9041] is in player's box
  (bind _asbp_third_person_character (Utilities|Casting|CastToBP_ThirdPersonCharacter OtherActor))
  (if (== (Variables|/Game/ThirdPerson/Blueprints/BP_ThirdPersonCharacter.BP_ThirdPersonCharacter_C|GetEnnemy_In_Box _asbp_third_person_character) self)
    (Variables|/Game/ThirdPerson/Blueprints/BP_ThirdPersonCharacter.BP_ThirdPersonCharacter_C|SetEnnemy_In_Box _asbp_third_person_character 0)))

(event Custom|Marker
  ;[1 0 0] Take damages
  (if (not (Variables|Common_conditions|GetInvincible%20?))
    (if (<= (Variables|HP|GetCurrent_Hit) (Variables|Common_conditions|GetHit_Numbers))
      (bind _result (Math|Float|IncrementFloat (Variables|HP|GetCurrent_Hit))
        (:%20%20
          (Variables|HP|SetCurrent_Hit _result)
          (CallFunction|Freeze)
          (CallFunction|HitEvent))))))

(event Custom|freeze_ordrer
  ;[0 0 0] For the childrens
)

(event Custom|hit_event
  ;[0 0 0] For the childrens
)

(event Custom|Finisher
  ;[0.8232 1 0] Finisher
  (if (Variables|Common_conditions|Getstopped?)
    (if (Variables|Common_conditions|GetCan%20be%20Killed?)
      (Utilities|FlowControl|DoOnce false
        (:Completed
          (bind _asbp_third_person_character (Utilities|Casting|CastToBP_ThirdPersonCharacter (Game|GetPlayerCharacter 0)))
          (if (== (Variables|/Game/ThirdPerson/Blueprints/BP_ThirdPersonCharacter.BP_ThirdPersonCharacter_C|GetEnnemy_In_Box _asbp_third_person_character) self)
            (Variables|/Game/ThirdPerson/Blueprints/BP_ThirdPersonCharacter.BP_ThirdPersonCharacter_C|SetEnnemy_In_Box _asbp_third_person_character 0)
            (CallFunction|Kill)
            (Variables|/Game/ThirdPerson/Blueprints/BP_ThirdPersonCharacter.BP_ThirdPersonCharacter_C|SetLocking? _asbp_third_person_character false)
            (Actor|DestroyActor)))))))

(event Custom|Freeze
  ;[1 1 1] Freeze when killed
  (if (>= (Variables|HP|GetCurrent_Hit) (Variables|Common_conditions|GetHit_Numbers))
    (Default|Update (Variables|HP|GetAs%20Marks))
    (bind _result (Math|Integer|IncrementInt (Variables|/Game/UI/Character_UI/Ennemies/WB_Marks.WB_Marks_C|GetLine (Variables|HP|GetAs%20Marks)))
      (:%20%20
        (Variables|/Game/UI/Character_UI/Ennemies/WB_Marks.WB_Marks_C|SetLine (Variables|HP|GetAs%20Marks) _result)
        (Variables|Common_conditions|Setstopped? true)
        (Components|Movement|StopMovementImmediately (Variables|Character|GetCharacterMovement))
        (Rendering|Material|SetMaterial (Variables|Character|GetMesh) 0 "/Game/StarterContent/Materials/M_Metal_Gold.M_Metal_Gold")
        (Variables|Common_conditions|SetCan%20be%20Killed? true)
        (CallFunction|FreezeOrdrer)
        (Development|PrintString "BOOOOOOOOOOOOOOOOOOOOOOOOOOOOOOOOOOOOOOOOOOOOOOOOOM")))
    (else
      (bind _aswb_marks (Utilities|Casting|CastToWB_Marks (UserInterface|GetWidget (Variables|Default|GetWidget))))
      (bind _output_get (Variables|HP|SetAs%20Marks _aswb_marks))
      (Default|Update _output_get)
      (bind _result_2 (Math|Integer|IncrementInt (Variables|/Game/UI/Character_UI/Ennemies/WB_Marks.WB_Marks_C|GetLine _output_get))
        (:%20%20
          (Variables|/Game/UI/Character_UI/Ennemies/WB_Marks.WB_Marks_C|SetLine _output_get _result_2))))))

(event EventBeginPlay
  ;[0.07005 0.9303 1] Begin play
  (bind _asbp_melia (Utilities|Casting|CastToBP_Melia (Game|GetPlayerCharacter 0)))
  (Variables|Default|SetAs%20BP%20Melia _asbp_melia)
  (bind _aswb_marks (Utilities|Casting|CastToWB_Marks (UserInterface|GetWidget (Variables|Default|GetWidget))))
  (Default|Init _aswb_marks (Variables|Common_conditions|GetHit_Numbers))
  (bind _aswb_marker_lock (Utilities|Casting|CastToWB_Marker_lock (UserInterface|GetWidget (Variables|Default|GetWidget1))))
  (Variables|Casts|SetAs%20Marker%20Lock _aswb_marker_lock)
  (Collision|SetCollisionResponsetoChannel (Variables|Collision|GetCapsuleComponent) "ECC_Camera" "ECR_Ignore"))

(event EventShotEvent
  ;[0 0 0] For the childrens
  (CallFunction|Marker)
  (CallFunction|Chase))

(fn ConstructionScript)