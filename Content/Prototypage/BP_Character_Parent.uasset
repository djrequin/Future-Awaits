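; Parent character Blueprint for interactable characters that open a dialog.
; On BeginPlay it copies its Name into TextToPrint and converts the CharacterName enum array into a string name list.
; Interaction creates a WB_Dialog_System widget once, adds it to the viewport and initializes it with the dialogs and names.
; Move_to_goal is an empty event, and overlap and Tick are disabled.
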(event Custom|Move_to_goal)

(event EventBeginPlay
  (|CallParentFunction)
  (Variables|Default|SetText%20to%20print (Variables|Default|GetName))
  (for _array_element (Variables|Default|GetCharacter_name)
    (Utilities|Array|Add (Variables|Default|GetNames_array) (Utilities|String|EnumtoString _array_element))))

(event Collision|EventActorBeginOverlap
  (params (OtherActor :type Actor%20Object%20Reference))
  (|CallParentFunction OtherActor) ; This node is disabled and will not be called.\nDrag off pins to build functionality.
)

(event EventTick
  (params (DeltaSeconds :type Float%20%28single-precision%29))
  (|CallParentFunction DeltaSeconds) ; This node is disabled and will not be called.\nDrag off pins to build functionality.
)

(event EventInteraction
  (Utilities|FlowControl|DoOnce false
    (:Completed
      (bind _returnvalue (UserInterface|CreateWidget "/Game/UI/Character_UI/WB_Dialog_System.WB_Dialog_System_C"))
      (UserInterface|Viewport|AddtoViewport _returnvalue 0)
      (Default|Init _returnvalue (Variables|Default|GetDialogs) (Variables|Default|GetNames_array)))))

(fn ConstructionScript
  (|CallParentFunction))